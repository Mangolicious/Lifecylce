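; Shard actor that scatters on spawn and bursts when BP_Jin touches it.
; BeginPlay picks one of three shard meshes at random, then pushes it with a radial impulse from a randomly offset origin near the actor so the launch direction varies.
; When BP_Jin overlaps the Sphere, it spawns an explosion particle effect at the mesh's location and destroys itself.
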(event `self.Sphere.OnComponentBeginOverlap`
  (params (OverlappedComponent :type "PrimitiveComponent Object Reference") (OtherActor :type "Actor Object Reference") (OtherComp :type "PrimitiveComponent Object Reference") (OtherBodyIndex :type Integer) (bFromSweep :type Boolean) (SweepResult :type "HitResult Structure (by ref)"))
  (cast `/Game/Prototype/Blueprints/BP_Jin` OtherActor)
  (`GameplayStatics.SpawnEmitterAtLocation` "/Game/Prototype/Particles/Shards/P_ShardExplosion.P_ShardExplosion" (`SceneComponent.K2_GetComponentLocation` (`self.StaticMesh`)))
  (`self.K2_DestroyActor`))

(event `self.ReceiveBeginPlay`
  (bind _staticmesh (`self.StaticMesh`))
  (switch `int` (`KismetMathLibrary.RandomIntegerInRange` 0 2)
    (:`0`
      (`StaticMeshComponent.SetStaticMesh` _staticmesh "/Game/Prototype/Particles/Shards/Shard1.Shard1"))
    (:`1`
      (`StaticMeshComponent.SetStaticMesh` _staticmesh "/Game/Prototype/Particles/Shards/Shard2.Shard2"))
    (:`2`
      (`StaticMeshComponent.SetStaticMesh` _staticmesh "/Game/Prototype/Particles/Shards/Shard3.Shard3")))
  (`PrimitiveComponent.AddRadialImpulse` _staticmesh (+ (`self.K2_GetActorLocation`) (`KismetMathLibrary.RandomUnitVector`)) 50.0 250.0 "RIF_Constant" false))

(fn `UserConstructionScript`)