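; Cloudscape actor that follows the player horizontally at a set cloud height and runs a day cycle with a lightning effect.
; Tick writes player location and sun color to a Material Parameter Collection.
; The DayCycle timeline drives the sun material, spring arm rotation, directional light and skylight.
; Five seconds after BeginPlay, a temporary blue directional light flashes through the Lightning timeline, then is destroyed after a short delay.
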(event `self.ReceiveTick`
  (params (DeltaSeconds :type "Float (single-precision)"))
  (bind _returnvalue (`GameplayStatics.GetPlayerCharacter` 0))
  (bind (_returnvalue_x _returnvalue_y) (`KismetMathLibrary.BreakVector` (`self.K2_GetActorLocation` _returnvalue)))
  (`self.K2_SetActorLocation` (`KismetMathLibrary.MakeVector` _returnvalue_x _returnvalue_y (`self.CloudHeight`)))
  (`KismetMaterialLibrary.SetVectorParameterValue` "/Game/Prototype/Meshes/Cloudmeshes/ParamaterCollection.ParamaterCollection" "Character Location" (`KismetMathLibrary.Conv_VectorToLinearColor` (`self.K2_GetActorLocation` _returnvalue)))
  (`KismetMaterialLibrary.SetVectorParameterValue` "/Game/Prototype/Meshes/Cloudmeshes/ParamaterCollection.ParamaterCollection" "Day Color" (stale `self.ReceiveBeginPlay` _sun_color)))

(event `self.ReceiveBeginPlay`
  (bind _sunlight (`self.Sunlight`))
  (bind _sun (`self.Sun`))
  (bind _lightcomponent (`SkyLight.LightComponent` (`self.Sky Light`)))
  (bind _lightcomponent_2 (`Light.LightComponent` _sunlight))
  (`|ExecutionSequence`
    (:`then_0`
      (bind _returnvalue (`PrimitiveComponent.CreateDynamicMaterialInstance` _sun 0 (`PrimitiveComponent.GetMaterial` _sun 0)))
      (bind _output_get (set `self.Sun Material` _returnvalue))
      (bind (_direction _pitch _yaw _directional_light_intensity _sky_light_intensity _sun_color _sky_color) (`Timeline|Day Cycle`)
        (:`Update`
          (`MaterialInstanceDynamic.SetVectorParameterValue` _output_get "Color In" _sun_color)
          (`MaterialInstanceDynamic.SetScalarParameterValue` _output_get "Intensity" 100.0)
          (`SceneComponent.K2_SetWorldRotation` (`self.SpringArm`) (`KismetMathLibrary.MakeRotator` 0.0 (* _pitch 5.0) _yaw) false false)
          (`self.K2_SetActorRotation` _sunlight (`KismetMathLibrary.MakeRotator` 0.0 _pitch _yaw) false)
          (`LightComponent.SetLightColor` _lightcomponent_2 _sun_color true)
          (`LightComponent.SetIntensity` _lightcomponent_2 _directional_light_intensity)
          (`SkyLightComponent.SetLightColor` _lightcomponent _sky_color)
          (`SkyLightComponent.SetIntensity` _lightcomponent _sky_light_intensity))))
    (:`then_1`
      ;[1 1 1] Thunder
      (`KismetSystemLibrary.Delay` 5.0)
      (bind _returnvalue_2 (`|SpawnActorFromClass` "/Script/Engine.DirectionalLight" (`KismetMathLibrary.MakeTransform` (0.0 0.0 0.0) (struct :`Pitch` -45.0 :`Yaw` 45.0)) "AlwaysSpawn" "OverrideRootScale" null null))
      (bind (_direction_2 _lighting) (`Timeline|Lightning`)
        (:`Update`
          (bind _lightcomponent_3 (`Light.LightComponent` _returnvalue_2))
          (`LightComponent.SetIntensity` _lightcomponent_3 _lighting)
          (`LightComponent.SetLightColor` _lightcomponent_3 (struct :`B` 1.0 :`A` 1.0) true)
          (`KismetSystemLibrary.Delay` 0.4)
          (`self.K2_DestroyActor` _returnvalue_2))))))

(fn `UserConstructionScript`)