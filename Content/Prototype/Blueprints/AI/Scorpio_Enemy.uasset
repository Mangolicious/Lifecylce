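; Scorpion enemy with a lock-on marker and a tail attack that damages and knocks back the player during an attack window.
; TakeDamage and AnyDamage both set Health to Damage minus Health, the latter on every update of its material-flash timeline.
; At zero or below, the next TakeDamage plays a sound, spawns random shard loot and destroys the actor.
; The montage and ragdoll death sequence is disconnected and never runs.
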(event `/Game/Prototype/Blueprints/AI/Combat_BPI.Take Damage`
  (params (Damage :type "Float (single-precision)") (`Bone Name` :type Name) (`Damage Causer` :type "Actor Object Reference") (Hit :type "HitResult Structure"))
  (bind _health (`self.Health`))
  (`/Engine/EditorBlueprintResources/StandardMacros.DoOnce` false :!label _label
    (:`Completed`
      (`KismetSystemLibrary.PrintString` (`KismetStringLibrary.Conv_NameToString` `Bone Name`))
      (`KismetSystemLibrary.PrintString` (`KismetSystemLibrary.GetDisplayName` `Damage Causer`))
      (if (<= (`self.Health`) 0.0)
        (`GameplayStatics.SpawnSoundAtLocation` "/Game/Prototype/Audio/SFX/Weapon/fuchteln_1.fuchteln_1" (`self.K2_GetActorLocation`) (struct) 1.0 1.0 0.0 null null)
        (`self.Spawn Loot`)
        (`KismetSystemLibrary.Delay` 2.0)
        (`self.K2_DestroyActor`)
        (`KismetSystemLibrary.PrintString` "Dead")
        (else
          (set `self.Health` (- Damage _health))
          (`KismetSystemLibrary.PrintString` (`KismetStringLibrary.Concat_StrStr` "Health: " (`KismetStringLibrary.Conv_DoubleToString` _health)))
          (`KismetSystemLibrary.Delay` 0.5)
          (goto _label :!via `Reset`))))))

(event `self.ReceiveBeginPlay`
  (`parent.ReceiveBeginPlay`)
  (`PrimitiveComponent.SetCollisionEnabled` (`self.Hitbox Tail`) "QueryAndPhysics")
  (`SkeletalMeshComponent.SetAllBodiesBelowSimulatePhysics` (`self.Mesh`) (`self.head_J`) true false)
  (bind _output_get (set `self.Health` (`.Health_35_99D0DCC24D20D4F76843D3A0ACA77F58` (break `/Game/Prototype/Blueprints/AI/EnemyBaseStats` (`self.Enemy Attribute`)))))
  (`KismetSystemLibrary.PrintString` (`KismetStringLibrary.Concat_StrStr` "Health: " (`KismetStringLibrary.Conv_DoubleToString` _output_get))))

(event `/Game/Prototype/Blueprints/AI/LockOnTarget_BPI.LockOnTarget`
  (bind _target_point (`self.Target Point`))
  (bind _isa (`/Engine/EditorBlueprintResources/StandardMacros.FlipFlop`)
    (:`A`
      (`SceneComponent.SetVisibility` _target_point _isa false))
    (:`B`
      (`SceneComponent.SetVisibility` _target_point _isa false))))

(event `Hit Event`
  (params (Target :type "PrimitiveComponent Object Reference"))
  (for _array_element (`PrimitiveComponent.GetOverlappingActors` Target "/Script/Engine.Pawn")
    (if (== _array_element "/Game/Prototype/Blueprints/PlayerCharacter/BP_Jin.BP_Jin")
      (`/Engine/EditorBlueprintResources/StandardMacros.DoOnce` false))))

(event `self.ReceiveAnyDamage`
  (params (Damage :type "Float (single-precision)") (DamageType :type "DamageType Object Reference") (InstigatedBy :type "Controller Object Reference") (DamageCauser :type "Actor Object Reference"))
  (bind _health (`self.Health`))
  (bind _mesh (`self.Mesh`))
  (`KismetSystemLibrary.PrintString` (`KismetStringLibrary.Conv_DoubleToString` Damage))
  (`PrimitiveComponent.CreateDynamicMaterialInstance` _mesh 1 "/Game/Prototype/Characters/ScorpioV2/M_ScorpioPlates_Inst.M_ScorpioPlates_Inst" "None")
  (bind (_direction _damage_flash) (`Timeline|Timeline_0` :!via `PlayFromStart`)
    (:`Update`
      (`MeshComponent.SetScalarParameterValueOnMaterials` _mesh "Flash" _damage_flash)
      (if (not (<= (`self.Health`) 0.0))
        (set `self.Health` (- Damage _health))
        (`KismetSystemLibrary.PrintString` (`KismetStringLibrary.Conv_DoubleToString` _health))))))

(event `self.ReceiveTick`
  (params (DeltaSeconds :type "Float (single-precision)")))

(event `Tail Attack Start`
  (set `self.Is Attacking?` true))

(event `self.Hitbox Tail.OnComponentBeginOverlap`
  (params (OverlappedComponent :type "PrimitiveComponent Object Reference") (OtherActor :type "Actor Object Reference") (OtherComp :type "PrimitiveComponent Object Reference") (OtherBodyIndex :type Integer) (bFromSweep :type Boolean) (SweepResult :type "HitResult Structure (by ref)"))
  (bind _returnvalue (`GameplayStatics.GetPlayerCharacter` 0))
  (bind (_bblockinghit _binitialoverlap _time _distance _location _impactpoint _normal _impactnormal _physmat _hitactor) (`GameplayStatics.BreakHitResult` SweepResult))
  (bind _charactermovement (`Character.CharacterMovement` (cast `/Game/Prototype/Blueprints/PlayerCharacter/BP_Jin` _returnvalue :!pure true)))
  (if (and (`self.Is Attacking?`) (== OtherActor _returnvalue))
    (`/Engine/EditorBlueprintResources/StandardMacros.DoOnce` false :!label _label_2
      (:`Completed`
        (`GameplayStatics.ApplyDamage` _hitactor 50.0)
        (`GameplayStatics.SpawnEmitterAtLocation` "/Game/Prototype/Particles/P_pulse.P_pulse" _impactpoint)
        (set `MovementComponent.Velocity` (0.0 0.0 0.0) _charactermovement)
        (`CharacterMovementComponent.AddImpulse` _charactermovement (* (`KismetMathLibrary.Normal` (+ (`self.K2_GetActorLocation` _hitactor) (`SceneComponent.K2_GetComponentLocation` (`self.Hitbox Tail`)))) 100.0) true)))))

(event `Tail Attack End`
  (set `self.Is Attacking?` false)
  (goto _label_2 :!via `Reset`))

(fn `Spawn Loot`
  (for _ (range (+ (`KismetMathLibrary.RandomIntegerInRange` (`self.Min Loot`) (`self.Max Loot`)) 1))
    (`|SpawnActorFromClass` "/Game/Prototype/Blueprints/WorldInteractive/Shard_BP.Shard_BP_C" (`self.GetTransform`) "AlwaysSpawn" "OverrideRootScale" null null)))

(fn `UserConstructionScript`
  (`parent.UserConstructionScript`))