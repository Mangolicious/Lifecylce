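; Base enemy Blueprint (Scorpio assets) that handles attacks, damage and death, taking its behavior tree and health in the Construction Script.
; AIAttack runs melee, charge or projectile attacks, with montage notifies driving hit traces, overlap damage and poise that blocks staggers.
; A Tick-fed gate turns it toward the player during attack montages.
; Death ragdolls it before destruction; an older loot-drop death chain is disconnected.
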(event `self.Sphere.OnComponentBeginOverlap`
  (params (OverlappedComponent :type "PrimitiveComponent Object Reference") (OtherActor :type "Actor Object Reference") (OtherComp :type "PrimitiveComponent Object Reference") (OtherBodyIndex :type Integer) (bFromSweep :type Boolean) (SweepResult :type "HitResult Structure (by ref)"))
  (if (`self.Hit Active`)
    (`/Engine/EditorBlueprintResources/StandardMacros.DoOnce` false :!label _label
      (:`Completed`
        (`GameplayStatics.ApplyDamage` OtherActor 500.0)
        (`KismetSystemLibrary.Delay` 1.0)
        (goto _label :!via `Reset`)))))

(event `/Game/Prototype/Blueprints/AI/Combat_BPI.Take Damage`
  (params (Damage :type "Float (single-precision)") (`Bone Name` :type Name) (`Damage Causer` :type "Actor Object Reference") (Hit :type "HitResult Structure"))
  (bind _mesh (`self.Mesh`))
  (bind _health (`self.Health`))
  (`KismetSystemLibrary.PrintString` (`KismetStringLibrary.Conv_DoubleToString` _health))
  (set `self.Health` (- _health Damage))
  (if (<= (`self.Health`) 0.0)
    (`KismetSystemLibrary.PrintString` (`KismetStringLibrary.Conv_DoubleToString` _health))
    (`|PlayMontage` (`self.Mesh`) (`self.Death Animation`)
      (:`OnNotifyBegin`
        (`PrimitiveComponent.SetCollisionObjectType` _mesh "ECC_PhysicsBody")
        (`SkeletalMeshComponent.SetAllBodiesSimulatePhysics` _mesh true)
        (`KismetSystemLibrary.Delay` 15.0)
        (`self.K2_DestroyActor`)))
    (elif (not (`self.Poise`))
      (`|PlayMontage` (`self.Mesh`) "/Game/Prototype/Characters/ScorpioV2/Scorpio_Stagger_Montage.Scorpio_Stagger_Montage"))))

(event `Attack Rotation`
  (bind _returnvalue (`self.K2_GetActorRotation`))
  (`self.K2_SetActorRotation` (`KismetMathLibrary.MakeRotator` (.roll _returnvalue) (.pitch _returnvalue) (.yaw (`KismetMathLibrary.RInterpTo` _returnvalue (`KismetMathLibrary.FindLookAtRotation` (`self.K2_GetActorLocation`) (`self.K2_GetActorLocation` (`GameplayStatics.GetPlayerCharacter` 0))) (`GameplayStatics.GetWorldDeltaSeconds`) (`self.Attack Rotation Rate`))))))

(event `self.ReceiveBeginPlay`
  (`GameplayStatics.SpawnEmitterAtLocation` (`self.Spawn FX`) (.location (`self.GetTransform`)) (.rotation (`self.GetTransform`)) (.scale (`self.GetTransform`)))
  (`SkeletalMeshComponent.SetAllBodiesBelowSimulatePhysics` (`self.Mesh`) "Head J" true false))

(event `/Game/Prototype/Blueprints/AI/Combat_BPI.AI Attack`
  (params (`Attack Animation` :type "AnimMontage Object Reference") (`Task Name` :type Name) (Attack :type "/Game/Prototype/Blueprints/AI/ActionType Enum" :default "NewEnumerator0"))
  (bind _returnvalue_location (`KismetMathLibrary.BreakTransform` (`self.GetTransform`)))
  (bind _returnvalue (+ (`self.K2_GetActorLocation`) (* (`self.GetActorForwardVector`) 50.0)))
  (set `self.Current Attack` Attack)
  (bind _output_get (set `self.Current Animation` `Attack Animation`))
  (`KismetSystemLibrary.PrintString` (`KismetSystemLibrary.GetDisplayName` _output_get))
  (switch `/Game/Prototype/Blueprints/AI/ActionType` Attack
    (:`NewEnumerator0`
      (bind _notifyname (`|PlayMontage` (`self.Mesh`) (`self.Current Animation`) 1.0 0.0 "Default" :!label _label_2)
        (:`then`
          (goto _label_4 :!via `Open`))
        (:`OnCompleted`
          (set `self.Poise` false :!label _label_3)
          (set `self.Hit Active` false)
          (set `CharacterMovementComponent.MaxWalkSpeed` 200.0 (`self.CharacterMovement`))
          (set `self.Current Animation` null))
        (:`OnInterrupted`
          (goto _label_4 :!via `Close`))
        (:`OnNotifyBegin`
          (switch `name` _notifyname
            (:`Hit`
              (set `self.Hit Active` true)
              (bind (_outhit _returnvalue_2) (`KismetSystemLibrary.SphereTraceSingleForObjects` :`Start` _returnvalue :`End` _returnvalue :`Radius` 100.0 :`ObjectTypes` (`|MakeArray` "ObjectTypeQuery3" :!type "EObjectTypeQuery Enum") :`DrawDebugType` "ForDuration" :`TraceColor` (struct :`R` 1.0 :`B` 0.632461 :`A` 1.0) :`DrawTime` 2.0))
              (if _returnvalue_2
                (`GameplayStatics.ApplyDamage` (`.HitActor` (`GameplayStatics.BreakHitResult` _outhit)) 250.0)))
            (:`Poise`
              (set `self.Poise` true))))
        (:`OnNotifyEnd`
          (switch `name` _notifyname
            (:`Hit`
              (goto _label_4 :!via `Close`))
            (:`Poise`
              (goto _label_3))))))
    (:`NewEnumerator2`
      (set `CharacterMovementComponent.MaxWalkSpeed` 500.0 (`self.CharacterMovement`))
      (goto _label_2))
    (:`NewEnumerator6`
      (`|SpawnActorFromClass` "/Game/Prototype/Blueprints/WorldInteractive/BP_Projectile.BP_Projectile_C" (`KismetMathLibrary.MakeTransform` _returnvalue_location (`KismetMathLibrary.Conv_VectorToRotator` (`SceneComponent.GetForwardVector` (`self.CapsuleComponent`)))) "Undefined" "OverrideRootScale" null null))))

(event `self.ReceiveTick`
  (params (DeltaSeconds :type "Float (single-precision)"))
  (`/Engine/EditorBlueprintResources/StandardMacros.Gate` true :!label _label_4
    (:`Exit`
      (`self.Attack Rotation`))))

(event `/Game/Prototype/Blueprints/AI/LockOnTarget_BPI.LockOnTarget`
  (bind _target_point (`self.Target Point`))
  ;[0.3594 0.07444 0.06729] Lock On
  (bind _isa (`/Engine/EditorBlueprintResources/StandardMacros.FlipFlop`)
    (:`A`
      (`SceneComponent.SetVisibility` _target_point _isa false))
    (:`B`
      (`SceneComponent.SetVisibility` _target_point _isa false))))

(event `Damage`
  (params (Damage :type "Float (double-precision)"))
  (set `self.Health` (- Damage (`self.Health`))))

(event `Death`
  (params (`Damage Causer` :type "Object Object Reference")))

(fn `UserConstructionScript`
  (bind _asenemy_aicontroller (cast `/Game/Prototype/Blueprints/AI/Enemy_AIController` (`self.GetController`)))
  (set `/Game/Prototype/Blueprints/AI/Enemy_AIController.Behavior Tree` "/Game/Prototype/Blueprints/AI/Scorpio_Behaviortree.Scorpio_Behaviortree" _asenemy_aicontroller)
  (set `self.Health` (`.Health_35_99D0DCC24D20D4F76843D3A0ACA77F58` (break `/Game/Prototype/Blueprints/AI/EnemyBaseStats` (`self.Enemy Attribute`)))))