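; AI controller for a prototype enemy that supplies player tracking data to its behavior tree.
; On BeginPlay it sets up Enemy_Blackboard and runs Enemy_Behaviortree.
; Every Tick it writes the controlled pawn's distance to player character 0, and that player's location, into the PlayerDistance and PlayerLocation blackboard keys, with no perception or validity checks.
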(event `self.ReceiveBeginPlay`
  (bind _blackboardcomponent (`self.UseBlackboard` "/Game/Prototype/Blueprints/AI/Enemy_Blackboard.Enemy_Blackboard"))
  (`self.RunBehaviorTree` "/Game/Prototype/Blueprints/AI/Enemy_Behaviortree.Enemy_Behaviortree"))

(event `self.ReceiveTick`
  (params (DeltaSeconds :type "Float (single-precision)"))
  (bind _returnvalue (`GameplayStatics.GetPlayerCharacter` 0))
  (`BlackboardComponent.SetValueAsFloat` (stale `self.ReceiveBeginPlay` _blackboardcomponent) (`self.Player Distance`) (`self.GetDistanceTo` (`self.K2_GetPawn`) _returnvalue))
  (`BlackboardComponent.SetValueAsVector` (stale `self.ReceiveBeginPlay` _blackboardcomponent) (`self.Player Location`) (`self.K2_GetActorLocation` _returnvalue)))

(fn `UserConstructionScript`)