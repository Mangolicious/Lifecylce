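; Enemy attack component that plays attack montages and applies melee hits to the player (BP_Jin), other pawns and destructibles.
; Attack plays the montage when IsDead is true, opening a gate that lets AttackRotationTick turn yaw toward the player until interruption or notify end.
; A "Hit" notify sphere-traces forward or along a custom line, skipping same-class actors unless FriendlyFire.
; Hits add impulses and call damage functions, but Damage and Radius inputs are unwired.
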(event `Attack Rotation Tick`
  (bind _character (`self.Character`))
  (bind _returnvalue (`Actor.K2_GetActorRotation` _character))
  (if (stale `Attack` `Rotation Adjust?`)
    (`/Engine/EditorBlueprintResources/StandardMacros.Gate` true :!label _label
      (:`Exit`
        (`Actor.K2_SetActorRotation` _character (`KismetMathLibrary.MakeRotator` (.roll _returnvalue) (.pitch _returnvalue) (.yaw (`KismetMathLibrary.RInterpTo` _returnvalue (`KismetMathLibrary.FindLookAtRotation` (`Actor.K2_GetActorLocation` _character) (`Actor.K2_GetActorLocation` (cast `/Game/Prototype/Blueprints/PlayerCharacter/BP_Jin` (`GameplayStatics.GetPlayerCharacter` 0) :!pure true))) (`GameplayStatics.GetWorldDeltaSeconds`) (`self.Attack Rotation Speed`)))) false)))))

(event `Attack`
  (params (AttackMontage :type "AnimMontage Object Reference") (Damage :type "Float (double-precision)" :default 25.0) (Radius :type "Float (double-precision)" :default 50.0) (Range :type "Float (double-precision)" :default 100.0) (`Friendly Fire?` :type Boolean) (`Rotation Adjust?` :type Boolean) (`Custom Trace?` :type Boolean) (`Trace Start` :type "Vector Structure") (`Trace End` :type "Vector Structure") (`Destructable Damage Intensity` :type "Float (double-precision)"))
  (bind _character (`self.Character`))
  (bind _character_2 (`self.Character`))
  (bind _returnvalue (`Actor.K2_GetActorLocation` _character_2))
  (set `self.Friendly Fire?` `Friendly Fire?`)
  (if (`self.IsDead?`)
    (bind _notifyname (`|PlayMontage` (`Character.Mesh` (`self.Character`)) (`self.Attack Montage`) (`self.Attack Speed`) 0.0 "Default")
      (:`then`
        (goto _label :!via `Open`))
      (:`OnInterrupted`
        (goto _label :!via `Close`))
      (:`OnNotifyBegin`
        (switch `name` _notifyname
          (:`Default`
            (`KismetSystemLibrary.PrintString` (`KismetStringLibrary.Concat_StrStr` "ERROR unknown play montage: " (`KismetStringLibrary.Conv_NameToString` "None")) true true (struct :`R` 1.0 :`A` 1.0) 20.0))
          (:`Hit`
            (if (not (`self.Friendly Fire?`))
              (bind _outactors (`GameplayStatics.GetAllActorsOfClass` (`GameplayStatics.GetObjectClass` (`self.Character`)))))
            (bind (_outhits _returnvalue_2) (`KismetSystemLibrary.SphereTraceMultiForObjects` (select `bool` `Custom Trace?` :`false` _returnvalue :`true` `Trace Start`) (select `bool` `Custom Trace?` :`false` (+ _returnvalue (* (`KismetMathLibrary.GetForwardVector` (`Actor.K2_GetActorRotation` _character_2)) Range)) :`true` (+ `Trace Start` (* `Trace End` Range))) 0.0 (`|MakeArray` "ObjectTypeQuery3" :!type "EObjectTypeQuery Enum") false _outactors "ForDuration" true (struct :`R` 1.0 :`A` 1.0) (struct :`G` 1.0 :`A` 1.0) 2.0))
            (if _returnvalue_2
              (for _array_element _outhits
                (bind (_bblockinghit _binitialoverlap _time _distance _location _impactpoint _normal _impactnormal _physmat _hitactor _hitcomponent) (`GameplayStatics.BreakHitResult` _array_element))
                (if _bblockinghit
                  (switch `ECollisionChannel` (`PrimitiveComponent.GetCollisionObjectType` _hitcomponent)
                    (:`ECC_Pawn`
                      (`/Engine/EditorBlueprintResources/StandardMacros.DoOnce` false :!label _label_2
                        (:`Completed`
                          (bind _asbp_jin (cast `/Game/Prototype/Blueprints/PlayerCharacter/BP_Jin` _hitactor)
                            (:`then`
                              (if (not (`/Game/Prototype/Blueprints/PlayerCharacter/BP_Jin.Is God Mode?` _asbp_jin))
                                (`CharacterMovementComponent.AddImpulse` (`Character.CharacterMovement` _asbp_jin) (+ (* (`Actor.GetActorForwardVector` (`self.Character`)) 1000.0) (0.0 0.0 500.0) (0.0 0.0 0.0)) true)
                                (`GameplayStatics.ApplyDamage` _hitactor 0.0 null _character)))
                            (:`CastFailed`
                              (`PrimitiveComponent.AddRadialImpulse` _hitcomponent _impactpoint 0.0 0.0 "RIF_Constant" false)
                              (`GameplayStatics.ApplyDamage` _hitactor 0.0 null _character))))))
                    (:`ECC_Destructible`
                      (`/Engine/EditorBlueprintResources/StandardMacros.DoOnce` false :!label _label_3
                        (:`Completed`
                          (`GameplayStatics.ApplyRadialDamage` :`BaseDamage` (* 0.0 (`self.Destructable Damage Intensity`)) :`Origin` _impactpoint :`DamageCauser` (`self.Character`) :`InstigatedByController` null :`DamagePreventionChannel` "ECC_Pawn")
                          (`PrimitiveComponent.AddRadialImpulse` _hitcomponent (0.0 0.0 0.0) 0.0 0.0 "RIF_Constant" false)))))))
              (`|ExecutionSequence`
                (:`then_0`
                  (goto _label_2 :!via `Reset`))
                (:`then_1`
                  (goto _label_3 :!via `Reset`)))))))
      (:`OnNotifyEnd`
        (goto _label :!via `Close`)))))