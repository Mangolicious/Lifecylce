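; Enemy spawner actor that spawns one enemy at its transform, either on play, on a repeating interval, or not at all.
; The construction script maps the chosen enemy type to a class, preview mesh, light color and name label; only Scorpio has a class.
; Each spawn is skipped while the current enemy is still valid, so interval mode acts as a respawn.
; Scorpio spawns also play an emitter effect.
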(event `self.ReceiveBeginPlay`
  (set `self.Current Enemy` null)
  (switch `/Game/Prototype/Blueprints/AI/SpawnCondition` (`self.Spawn Condition`)
    (:`NewEnumerator0`
      (`self.Spawn`))
    (:`NewEnumerator1`
      (`KismetSystemLibrary.K2_SetTimerDelegate` (delegate `Spawn`) (`self.Respawn Time`) true))
    (:`NewEnumerator2`
      (`KismetSystemLibrary.PrintString` "Spawn Blocked" true true (struct :`R` 1.0 :`B` 0.028497 :`A` 1.0)))))

(event `Spawn`
  (`/Engine/EditorBlueprintResources/StandardMacros.IsValid` (`self.Current Enemy`)
    (:`Is Not Valid`
      (bind _returnvalue (`|SpawnActorFromClass` (`self.Enemy Class`) (`self.GetTransform`) (`self.Collision Debug`) "OverrideRootScale" null null))
      (set `self.Current Enemy` _returnvalue)
      (switch `/Game/Prototype/Blueprints/AI/EnemyType` (`self.Enemy`)
        (:`NewEnumerator1`
          (`GameplayStatics.SpawnEmitterAtLocation` null))))))

(fn `UserConstructionScript`
  (bind _preview_mesh (`self.Preview Mesh`))
  (`|ExecutionSequence`
    (:`then_0`
      (switch `/Game/Prototype/Blueprints/AI/EnemyType` (`self.Enemy`)
        (:`NewEnumerator1`
          (set `self.Enemy Class` "/Game/Prototype/Blueprints/AI/Scorpio_Enemy.Scorpio_Enemy_C")
          (`SkinnedMeshComponent.SetSkinnedAssetAndUpdate` _preview_mesh "/Game/Prototype/Characters/ScorpioV2/Scorpio_Character.Scorpio_Character" true)
          (`LightComponent.SetLightColor` (`self.Editor Light`) (struct :`R` 0.204612 :`B` 1.0 :`A` 1.0) true))
        (:`NewEnumerator2`
          (set `self.Enemy Class` null)
          (`SkinnedMeshComponent.SetSkinnedAssetAndUpdate` _preview_mesh null true)
          (`LightComponent.SetLightColor` (`self.Editor Light`) (struct :`R` 1.0 :`G` 0.276147 :`A` 1.0) true)
          (`KismetSystemLibrary.PrintString` "Not Available"))
        (:`NewEnumerator3`
          (set `self.Enemy Class` null)
          (`KismetSystemLibrary.PrintString` "Not Available"))
        (:`NewEnumerator4`
          (set `self.Enemy Class` null)
          (`KismetSystemLibrary.PrintString` "Not Available"))))
    (:`then_1`
      (`TextRenderComponent.K2_SetText` (`self.Enemy Name`) (`KismetTextLibrary.Conv_StringToText` (`|GetEnumeratorNameAsString` (`self.Enemy`)))))))