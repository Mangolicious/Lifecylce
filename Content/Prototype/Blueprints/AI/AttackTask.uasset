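; Behavior tree task that makes an AI pawn implementing Combat_BPI perform an attack from AttackArray.
; AttackBehavior selects the first entry or a random one, sent via AIAttackMessage with a built task name, then the task waits the animation's length before finishing successfully.
; Random picks are separate calls that exclude the last entry, so attack, name and delay can mismatch.
; Other pawns only print "Wrong Pawn", leaving the task unfinished.
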(event `self.ReceiveExecuteAI`
  (params (OwnerController :type "AIController Object Reference") (ControlledPawn :type "Pawn Object Reference"))
  (bind _attack_array (`self.Attack Array`))
  (bind _output (`|GetArrayItem` _attack_array))
  (bind (_attacktype _animation) (break `/Game/Prototype/Blueprints/AI/AttackStruct` _output))
  (bind _output_2 (`|GetArrayItem` _attack_array (`KismetMathLibrary.RandomInteger` (- (`KismetArrayLibrary.Array_Length` _attack_array) 1))))
  (bind (_attacktype_2 _animation_2) (break `/Game/Prototype/Blueprints/AI/AttackStruct` _output_2))
  (if (`KismetSystemLibrary.DoesImplementInterface` ControlledPawn "/Game/Prototype/Blueprints/AI/Combat_BPI.Combat_BPI_C")
    (switch `/Game/Prototype/Blueprints/AI/AttackBehaviorType` (`self.Attack Behavior`)
      (:`NewEnumerator1`
        (message `/Game/Prototype/Blueprints/AI/Combat_BPI.AI Attack` ControlledPawn _output (`KismetStringLibrary.Conv_StringToName` (`KismetStringLibrary.Concat_StrStr` (`|GetEnumeratorNameAsString` _attacktype) " " (`KismetStringLibrary.Conv_NameToString` (`self.Attack Name`)))))
        (bind _returnvalue (`AnimSequenceBase.GetPlayLength` _animation))
        (`KismetSystemLibrary.Delay` _returnvalue))
      (:`NewEnumerator0`
        (message `/Game/Prototype/Blueprints/AI/Combat_BPI.AI Attack` ControlledPawn _output_2 (`KismetStringLibrary.Conv_StringToName` (`KismetStringLibrary.Concat_StrStr` (`|GetEnumeratorNameAsString` _attacktype_2) " " "Random")))
        (bind _returnvalue_2 (`AnimSequenceBase.GetPlayLength` _animation_2))
        (`KismetSystemLibrary.Delay` _returnvalue_2)))
    (`self.FinishExecute` true)
    (else
      (`KismetSystemLibrary.PrintString` "Wrong Pawn" true true (struct :`R` 1.0 :`B` 0.263523 :`A` 1.0)))))