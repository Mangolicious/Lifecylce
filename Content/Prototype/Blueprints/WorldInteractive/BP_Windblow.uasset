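; BP_Windblow is a world-interactive wind gust that pushes the player character, BP_Jin, along its arrow's direction.
; Overlapping the Proximity component starts the Blow timeline, whose event checks whether Jin is inside the Box.
; If so, it spawns a wind particle sized to the Box extent and plays an intensity timeline that applies scaled velocity-change impulses.
; Ground friction is zeroed during the push and set to one afterward.
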(event `self.Box.OnComponentEndOverlap`
  (params (OverlappedComponent :type "PrimitiveComponent Object Reference") (OtherActor :type "Actor Object Reference") (OtherComp :type "PrimitiveComponent Object Reference") (OtherBodyIndex :type Integer))
  (set `self.Player in Range?` false))

(event `self.Box.OnComponentBeginOverlap`
  (params (OverlappedComponent :type "PrimitiveComponent Object Reference") (OtherActor :type "Actor Object Reference") (OtherComp :type "PrimitiveComponent Object Reference") (OtherBodyIndex :type Integer) (bFromSweep :type Boolean) (SweepResult :type "HitResult Structure (by ref)"))
  (`/Engine/EditorBlueprintResources/StandardMacros.IsValid` OtherActor
    (:`Is Valid`
      (bind _asbp_jin (cast `/Game/Prototype/Blueprints/PlayerCharacter/BP_Jin` OtherActor))
      (set `self.Player in Range?` true))))

(event `self.Proximity.OnComponentBeginOverlap`
  (params (OverlappedComponent :type "PrimitiveComponent Object Reference") (OtherActor :type "Actor Object Reference") (OtherComp :type "PrimitiveComponent Object Reference") (OtherBodyIndex :type Integer) (bFromSweep :type Boolean) (SweepResult :type "HitResult Structure (by ref)"))
  (`/Engine/EditorBlueprintResources/StandardMacros.IsValid` OtherActor
    (:`Is Valid`
      (`KismetSystemLibrary.PrintString` "Wind Active")
      (`Timeline|Blow` :!via `PlayFromStart`
        (:`Blow`
          (if (`self.Player in Range?`)
            (bind _returnvalue (`GameplayStatics.SpawnEmitterAtLocation` "/Game/Prototype/Particles/P_WindBlow.P_WindBlow" (`SceneComponent.K2_GetComponentLocation` (`self.Arrow`)) (struct :`Yaw` -90.0)))
            (`ParticleSystemComponent.SetVectorParameter` _returnvalue "Size" (`BoxComponent.BoxExtent` (`self.Box`)))
            (bind (_direction _wind_intensity) (`Timeline|Wind Inensity` :!via `PlayFromStart`)
              (:`Update`
                (bind _charactermovement (`Character.CharacterMovement` (stale `self.Box.OnComponentBeginOverlap` _asbp_jin)))
                (set `CharacterMovementComponent.GroundFriction` 0.0 _charactermovement)
                (`CharacterMovementComponent.AddImpulse` _charactermovement (* (`SceneComponent.GetForwardVector` (`self.Arrow`)) (* _wind_intensity (`self.Blow Intensity`))) true))
              (:`Finished`
                (set `CharacterMovementComponent.GroundFriction` 1.0 _charactermovement)))))))))

(fn `UserConstructionScript`)