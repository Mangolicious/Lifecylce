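; FlowVolume is a world-interactive volume that pushes the BP_Jin player along its Arrow's forward direction.
; On Box begin overlap it stores the player and plays a timeline, whose updates repeatedly add a mass-dependent impulse, scaled by Force, to the character movement.
; Any end overlap on the Box stops the timeline and the push, without checking which actor left.
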(event `self.Box.OnComponentBeginOverlap`
  (params (OverlappedComponent :type "PrimitiveComponent Object Reference") (OtherActor :type "Actor Object Reference") (OtherComp :type "PrimitiveComponent Object Reference") (OtherBodyIndex :type Integer) (bFromSweep :type Boolean) (SweepResult :type "HitResult Structure (by ref)"))
  (`/Engine/EditorBlueprintResources/StandardMacros.IsValid` OtherActor
    (:`Is Valid`
      (bind _asbp_jin (cast `/Game/Prototype/Blueprints/PlayerCharacter/BP_Jin` OtherActor))
      (bind _output_get (set `self.Player` _asbp_jin))
      (`Timeline|Timeline_0` :!label _label
        (:`Update`
          (`CharacterMovementComponent.AddImpulse` (`Character.CharacterMovement` _output_get) (* (+ (`SceneComponent.GetForwardVector` (`self.Arrow`)) (0.0 0.0 0.0)) (`self.Force`)) false))))))

(event `self.Box.OnComponentEndOverlap`
  (params (OverlappedComponent :type "PrimitiveComponent Object Reference") (OtherActor :type "Actor Object Reference") (OtherComp :type "PrimitiveComponent Object Reference") (OtherBodyIndex :type Integer))
  (goto _label :!via `Stop`))

(fn `UserConstructionScript`)