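; FireworkBox_BP is an interactive world prop that launches fireworks when the BP_Jin character overlaps its Box component.
; The overlap plays the Firework timeline, whose Fire event track spawns a BP_Rocket at the box's location.
; Each rocket gets a slightly varied scale and a random roll, pitch and yaw within a symmetric range set by the Random variable.
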(event `self.Box.OnComponentBeginOverlap`
  (params (OverlappedComponent :type "PrimitiveComponent Object Reference") (OtherActor :type "Actor Object Reference") (OtherComp :type "PrimitiveComponent Object Reference") (OtherBodyIndex :type Integer) (bFromSweep :type Boolean) (SweepResult :type "HitResult Structure (by ref)"))
  (bind _random (`self.Random`))
  (bind _returnvalue (* -1 _random))
  (`/Engine/EditorBlueprintResources/StandardMacros.IsValid` OtherActor
    (:`Is Valid`
      (cast `/Game/Prototype/Blueprints/PlayerCharacter/BP_Jin` OtherActor)
      (`Timeline|Firework`
        (:`Fire`
          (`|SpawnActorFromClass` "/Game/Prototype/Blueprints/WorldInteractive/BP_Rocket.BP_Rocket_C" (`KismetMathLibrary.MakeTransform` (`self.K2_GetActorLocation`) (`KismetMathLibrary.MakeRotator` (`KismetMathLibrary.RandomFloatInRange` _random _returnvalue) (`KismetMathLibrary.RandomFloatInRange` _random _returnvalue) (`KismetMathLibrary.RandomFloatInRange` _random _returnvalue)) (`KismetMathLibrary.Conv_DoubleToVector` (`KismetMathLibrary.RandomFloatInRange` 1.0 1.2))) "Undefined" "OverrideRootScale" null null))))))

(fn `UserConstructionScript`)