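; BP_Fireballshooter is a stationary-logic hazard that fires BP_Projectile at the player while BP_Jin is inside its attack sphere.
; The construction script sizes the sphere from AttackRadius, and overlap events start or stop Timeline_0.
; The timeline acts as a repeating fire timer: each finish spawns a projectile aimed at player character 0's current location, then restarts while BP_Jin stays in range.
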(event `self.Sphere.OnComponentBeginOverlap`
  (params (OverlappedComponent :type "PrimitiveComponent Object Reference") (OtherActor :type "Actor Object Reference") (OtherComp :type "PrimitiveComponent Object Reference") (OtherBodyIndex :type Integer) (bFromSweep :type Boolean) (SweepResult :type "HitResult Structure (by ref)"))
  (cast `/Game/Prototype/Blueprints/PlayerCharacter/BP_Jin` OtherActor)
  (set `self.Is In Range?` true)
  (`Timeline|Timeline_0` :!via `PlayFromStart` :!label _label
    (:`Finished`
      (`|SpawnActorFromClass` "/Game/Prototype/Blueprints/WorldInteractive/BP_Projectile.BP_Projectile_C" (`KismetMathLibrary.MakeTransform` (`self.K2_GetActorLocation`) (`KismetMathLibrary.FindLookAtRotation` (`self.K2_GetActorLocation`) (`self.K2_GetActorLocation` (`GameplayStatics.GetPlayerCharacter` 0)))) "Undefined" "OverrideRootScale" null null)
      (if (`self.Is In Range?`)
        (goto _label :!via `PlayFromStart`)))))

(event `self.Sphere.OnComponentEndOverlap`
  (params (OverlappedComponent :type "PrimitiveComponent Object Reference") (OtherActor :type "Actor Object Reference") (OtherComp :type "PrimitiveComponent Object Reference") (OtherBodyIndex :type Integer))
  (cast `/Game/Prototype/Blueprints/PlayerCharacter/BP_Jin` OtherActor)
  (set `self.Is In Range?` false)
  (goto _label :!via `Stop`))

(fn `UserConstructionScript`
  (`SphereComponent.SetSphereRadius` (`self.Sphere`) (`self.Attack Radius`) true))