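; BP_Projectile is a prototype projectile that explodes, deals damage and destroys itself when its Sphere overlaps something.
; The overlapped component's collision object type selects the damage mode after spawning an explosion emitter.
; Pawns take direct damage, while world static, world dynamic, destructible and projectile hits apply radial damage that ignores the first player's character.
; The Sphere hit event and construction script are empty.
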(event `self.Sphere.OnComponentBeginOverlap`
  (params (OverlappedComponent :type "PrimitiveComponent Object Reference") (OtherActor :type "Actor Object Reference") (OtherComp :type "PrimitiveComponent Object Reference") (OtherBodyIndex :type Integer) (bFromSweep :type Boolean) (SweepResult :type "HitResult Structure (by ref)"))
  (bind _returnvalue (`self.K2_GetActorLocation`))
  (bind _damage (`self.Damage`))
  (bind _damage_type (`self.Damage Type`))
  (switch `ECollisionChannel` (`PrimitiveComponent.GetCollisionObjectType` OtherComp)
    (:`ECC_WorldStatic`
      (`GameplayStatics.SpawnEmitterAtLocation` "/Game/Prototype/Particles/P_Explosion.P_Explosion" _returnvalue :!label _label)
      (`GameplayStatics.ApplyRadialDamage` _damage _returnvalue (`self.Radius`) _damage_type (`|MakeArray` (`GameplayStatics.GetPlayerCharacter` 0) :!type "Actor Object Reference") self null))
    (:`ECC_WorldDynamic`
      (goto _label))
    (:`ECC_Pawn`
      (`GameplayStatics.SpawnEmitterAtLocation` "/Game/Prototype/Particles/P_Explosion.P_Explosion" _returnvalue)
      (`GameplayStatics.ApplyDamage` OtherActor _damage null self _damage_type))
    (:`ECC_Destructible`
      (goto _label))
    (:`ECC_GameTraceChannel1`
      (goto _label)))
  (`self.K2_DestroyActor`))

(event `self.Sphere.OnComponentHit`
  (params (HitComponent :type "PrimitiveComponent Object Reference") (OtherActor :type "Actor Object Reference") (OtherComp :type "PrimitiveComponent Object Reference") (NormalImpulse :type "Vector Structure") (Hit :type "HitResult Structure (by ref)")))

(fn `UserConstructionScript`)