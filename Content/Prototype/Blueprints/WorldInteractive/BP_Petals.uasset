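; BP_Petals is an interactive world effect whose Niagara petals respond to the player character's position and movement.
; A Sphere overlap by any actor switches IsActive on, and ending an overlap switches it off.
; While active, Tick feeds Niagara user parameters: a negated, speed-scaled MovementForce, the player's location offset down toward the feet, and Force from BP_Jin's NiagaraForce.
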(event `self.ReceiveTick`
  (params (DeltaSeconds :type "Float (single-precision)"))
  (bind _returnvalue (`GameplayStatics.GetPlayerCharacter` 0))
  (bind _niagara (`self.Niagara`))
  (if (`self.Is Active?`)
    (`NiagaraComponent.SetNiagaraVariableFloat` _niagara "User.MovementForce" (* (/ (`KismetMathLibrary.VSize` (`self.GetVelocity` _returnvalue)) 200.0) -1.0))
    (`NiagaraComponent.SetNiagaraVariableVec3` _niagara "User.PlayerLocation" (+ (`self.K2_GetActorLocation` _returnvalue) (0.0 0.0 -88.0)))
    (bind _asbp_jin (cast `/Game/Prototype/Blueprints/PlayerCharacter/BP_Jin` _returnvalue))
    (`NiagaraComponent.SetNiagaraVariableFloat` _niagara "User.Force" (`/Game/Prototype/Blueprints/PlayerCharacter/BP_Jin.Niagara Force` _asbp_jin))))

(event `self.Sphere.OnComponentBeginOverlap`
  (params (OverlappedComponent :type "PrimitiveComponent Object Reference") (OtherActor :type "Actor Object Reference") (OtherComp :type "PrimitiveComponent Object Reference") (OtherBodyIndex :type Integer) (bFromSweep :type Boolean) (SweepResult :type "HitResult Structure (by ref)"))
  (set `self.Is Active?` true))

(event `self.Sphere.OnComponentEndOverlap`
  (params (OverlappedComponent :type "PrimitiveComponent Object Reference") (OtherActor :type "Actor Object Reference") (OtherComp :type "PrimitiveComponent Object Reference") (OtherBodyIndex :type Integer))
  (set `self.Is Active?` false))

(fn `UserConstructionScript`)