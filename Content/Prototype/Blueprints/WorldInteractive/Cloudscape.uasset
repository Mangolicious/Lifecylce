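; Cloudscape actor that drives the day cycle and keeps a cloud layer under or around the player at a set height.
; DayCycle timeline orbits the sun on a spring arm and updates sunlight, skylight and fog.
; A material parameter collection receives light, wind-driven cloud speed and character location.
; Touching CloudLayer respawns and kills BP_Jin with a cloud effect, pausing follow for seven seconds; the lightning branch is disabled.
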(event `self.CloudLayer.OnComponentBeginOverlap`
  (params (OverlappedComponent :type "PrimitiveComponent Object Reference") (OtherActor :type "Actor Object Reference") (OtherComp :type "PrimitiveComponent Object Reference") (OtherBodyIndex :type Integer) (bFromSweep :type Boolean) (SweepResult :type "HitResult Structure (by ref)"))
  (bind _asbp_jin (cast `/Game/Prototype/Blueprints/PlayerCharacter/BP_Jin` OtherActor))
  (`/Game/Prototype/Blueprints/PlayerCharacter/BP_Jin.Respawn` _asbp_jin)
  (`/Game/Prototype/Blueprints/PlayerCharacter/BP_Jin.Death` _asbp_jin)
  (`GameplayStatics.SpawnEmitterAtLocation` "/Game/Prototype/Particles/P_Cloud.P_Cloud" (+ (`self.K2_GetActorLocation` _asbp_jin) (0.0 0.0 -200.0)))
  (set `self.Is Respawning` true)
  (`KismetSystemLibrary.Delay` 7.0)
  (set `self.Is Respawning` false))

(event `self.ReceiveTick`
  (params (DeltaSeconds :type "Float (single-precision)"))
  (bind _returnvalue (`GameplayStatics.GetPlayerCharacter` 0))
  (bind (_returnvalue_x _returnvalue_y) (`KismetMathLibrary.BreakVector` (`self.K2_GetActorLocation` _returnvalue)))
  (`KismetMaterialLibrary.SetVectorParameterValue` "/Game/Prototype/Environment/Clouds/Lijar_ParamaterCollection.Lijar_ParamaterCollection" "Day Color" (stale `self.ReceiveBeginPlay` _sky_light_color))
  (`KismetMaterialLibrary.SetVectorParameterValue` "/Game/Prototype/Environment/Clouds/Lijar_ParamaterCollection.Lijar_ParamaterCollection" "Light Vector" (`KismetMathLibrary.Conv_VectorToLinearColor` (`KismetMathLibrary.Conv_RotatorToVector` (`KismetMathLibrary.MakeRotator` 0.0 (stale `self.ReceiveBeginPlay` _pitch) (stale `self.ReceiveBeginPlay` _yaw)))))
  (`KismetMaterialLibrary.SetScalarParameterValue` "/Game/Prototype/Environment/Clouds/Lijar_ParamaterCollection.Lijar_ParamaterCollection" "Light Intensity" (stale `self.ReceiveBeginPlay` _star_brightness))
  (`/Engine/EditorBlueprintResources/StandardMacros.IsValid` _returnvalue
    (:`Is Valid`
      (if (not (`self.Is Respawning`))
        (`self.K2_SetActorLocation` (`KismetMathLibrary.MakeVector` _returnvalue_x _returnvalue_y (`self.CloudHeight`))))
      (`KismetMaterialLibrary.SetVectorParameterValue` "/Game/Prototype/Environment/Clouds/Lijar_ParamaterCollection.Lijar_ParamaterCollection" "Character Location" (`KismetMathLibrary.Conv_VectorToLinearColor` (`self.K2_GetActorLocation` _returnvalue))))))

(event `self.ReceiveBeginPlay`
  (bind _sunlight (`self.Sunlight`))
  (bind _sun (`self.Sun`))
  (bind _component (`ExponentialHeightFog.Component` (`self.Fog`)))
  (bind _lightcomponent (`SkyLight.LightComponent` (`self.Sky Light`)))
  (bind _lightcomponent_2 (`Light.LightComponent` _sunlight))
  (`|ExecutionSequence`
    (:`then_0`
      (bind _returnvalue (`PrimitiveComponent.CreateDynamicMaterialInstance` _sun 0 (`PrimitiveComponent.GetMaterial` _sun 0) "None"))
      (bind _output_get (set `self.Sun Material` _returnvalue))
      (bind (_direction _pitch _yaw _directional_light_intensity _sky_light_intensity _star_brightness _sun_color _sky_light_color) (`Timeline|Day Cycle` :`NewTime` (`self.Start Time`) :!label _label)
        (:`Update`
          (`MaterialInstanceDynamic.SetVectorParameterValue` _output_get "Color In" (* _sun_color (`self.Sun Brightness`)))
          (`MaterialInstanceDynamic.SetScalarParameterValue` _output_get "Intensity" (`self.Sun Intesity`))
          (`SceneComponent.K2_SetWorldRotation` (`self.SpringArm`) (`KismetMathLibrary.MakeRotator` 0.0 (* _pitch 5.0) _yaw) false false)
          (`|ExecutionSequence`
            (:`then_0`
              (`self.K2_SetActorRotation` _sunlight (`KismetMathLibrary.FindLookAtRotation` (`SceneComponent.K2_GetComponentLocation` (`self.SunTop`)) (`SceneComponent.K2_GetComponentLocation` (`self.DefaultSceneRoot`))) false)
              (`LightComponent.SetLightColor` _lightcomponent_2 _sun_color true)
              (`LightComponent.SetIntensity` _lightcomponent_2 _directional_light_intensity)
              (`SkyLightComponent.SetLightColor` _lightcomponent _sky_light_color)
              (`SkyLightComponent.SetIntensity` _lightcomponent _sky_light_intensity))
            (:`then_1`
              (`ExponentialHeightFogComponent.SetFogInscatteringColor` _component _sky_light_color)
              (`ExponentialHeightFogComponent.SetFogMaxOpacity` _component (+ (* _star_brightness -1.0) 1.0)))))))
    (:`then_1`
      ;[0 0.9903 1] Thunder
      (`KismetSystemLibrary.Delay` 5.0)
      (if (not true)
        (bind _returnvalue_2 (`|SpawnActorFromClass` "/Script/Engine.DirectionalLight" (`KismetMathLibrary.MakeTransform` (0.0 0.0 0.0) (struct :`Pitch` -45.0 :`Yaw` 45.0)) "AlwaysSpawn" "OverrideRootScale" null null))
        (bind (_direction_2 _lighting) (`Timeline|Lightning`)
          (:`Update`
            (bind _lightcomponent_3 (`Light.LightComponent` _returnvalue_2))
            (`LightComponent.SetIntensity` _lightcomponent_3 _lighting)
            (`LightComponent.SetLightColor` _lightcomponent_3 (struct :`B` 1.0 :`A` 1.0) true)
            (`KismetSystemLibrary.Delay` 0.4)
            (`self.K2_DestroyActor` _returnvalue_2)))))
    (:`then_2`
      (goto _label :!via `SetNewTime`))
    (:`then_3`
      (`TimelineComponent.SetPlayRate` (`self.Day Cycle`) (`self.Play Rate`)))
    (:`then_4`
      (`KismetMaterialLibrary.SetVectorParameterValue` "/Game/Prototype/Environment/Clouds/Lijar_ParamaterCollection.Lijar_ParamaterCollection" "Cloud Speed" (`KismetMathLibrary.Conv_VectorToLinearColor` (* (`self.Cloud Direction`) (`WindDirectionalSourceComponent.Speed` (`WindDirectionalSource.Component` (`self.Wind Actor`)))))))))

(fn `UserConstructionScript`)