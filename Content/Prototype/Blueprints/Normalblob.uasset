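; Normalblob is a prototype actor that feeds a world location into its Sphere's material, starting with its own position at construction.
; Every tick it gets all Normalblob actors and line-traces from itself to each one, with timed debug drawing.
; When a trace hits its intended blob, it stores that actor and passes that blob's sphere location to its own "World Location" parameter, so the last match wins.
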(event `self.ReceiveTick`
  (params (DeltaSeconds :type "Float (single-precision)"))
  (bind _outactors (`GameplayStatics.GetAllActorsOfClass` "Normalblob_C"))
  (for _array_element _outactors
    (bind _outhit (`KismetSystemLibrary.LineTraceSingleForObjects` :`Start` (`self.K2_GetActorLocation`) :`End` (`self.K2_GetActorLocation` _array_element) :`ObjectTypes` (`|MakeArray` "ObjectTypeQuery1" "ObjectTypeQuery2" :!type "EObjectTypeQuery Enum") :`DrawDebugType` "ForDuration"))
    (bind (_bblockinghit _binitialoverlap _time _distance _location _impactpoint _normal _impactnormal _physmat _hitactor) (`GameplayStatics.BreakHitResult` _outhit))
    (if (== _array_element _hitactor)
      (set `self.Actor` _hitactor)
      (`MeshComponent.SetVectorParameterValueOnMaterials` (`self.Sphere`) "World Location" (`SceneComponent.K2_GetComponentLocation` (`/Game/Prototype/Blueprints/Normalblob.Sphere` _array_element))))))

(fn `UserConstructionScript`
  (`MeshComponent.SetVectorParameterValueOnMaterials` (`self.Sphere`) "World Location" (`SceneComponent.K2_GetComponentLocation` (`self.Sphere`))))