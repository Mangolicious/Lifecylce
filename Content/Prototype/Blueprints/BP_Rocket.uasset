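; Firework rocket actor that launches via ProjectileMovement and bursts into a Hanabi particle effect after a short random flight.
; The construction script randomizes the initial speed and picks one of two rocket meshes.
; BeginPlay sets InitialSpeed again from a lower random range, waits a random delay, then spawns one of three randomly scaled emitters at its location and destroys the actor.
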(event `self.ReceiveBeginPlay`
  (bind _returnvalue (`KismetMathLibrary.RandomFloatInRange` 1.0 2.0))
  (set `ProjectileMovementComponent.InitialSpeed` (* _returnvalue 1000.0) (`self.ProjectileMovement`))
  (`KismetSystemLibrary.Delay` (- _returnvalue 0.2))
  (`GameplayStatics.SpawnEmitterAtLocation` (select `int` (`KismetMathLibrary.RandomIntegerInRange` 0 2) :`0` "/Game/Prototype/Particles/P_Hanabi.P_Hanabi" :`1` "/Game/Prototype/Particles/P_Hanabi1.P_Hanabi1" :`2` "/Game/Prototype/Particles/P_Hanabi2.P_Hanabi2" :!type "ParticleSystem Object Reference") (`self.K2_GetActorLocation`) (struct) (`KismetMathLibrary.Conv_DoubleToVector` (`KismetMathLibrary.RandomFloatInRange` 1.0 2.0)))
  (`self.K2_DestroyActor`))

(fn `UserConstructionScript`
  (bind _staticmesh (`self.StaticMesh`))
  (set `ProjectileMovementComponent.InitialSpeed` (`KismetMathLibrary.RandomFloatInRange` 2000.0 3000.0) (`self.ProjectileMovement`))
  (switch `int` (`KismetMathLibrary.RandomIntegerInRange` 0 1)
    (:`0`
      (`StaticMeshComponent.SetStaticMesh` _staticmesh "/Game/Prototype/Particles/Meshes/Rocket01.Rocket01"))
    (:`1`
      (`StaticMeshComponent.SetStaticMesh` _staticmesh "/Game/Prototype/Particles/Meshes/Rocket02.Rocket02"))))