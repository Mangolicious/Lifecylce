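; Menu control Blueprint that arms its mesh with a Spirit Katana and provides a left/right test relative to a spline.
; BeginPlay spawns the katana and attaches it to the R_Hand socket of the mesh.
; CheckLeftRight takes the dot-product angle between the spline's right vector and the direction from the spline point to the actor, returning true when it exceeds a given degree range.
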(event `self.ReceiveBeginPlay`
  (bind _returnvalue (`|SpawnActorFromClass` "/Game/Prototype/Blueprints/PlayerCharacter/BP_Spiritkatana.BP_Spiritkatana_C" (`KismetMathLibrary.MakeTransform` (0.0 0.0 0.0)) "AlwaysSpawn" "OverrideRootScale" null null))
  (`self.K2_AttachToComponent` _returnvalue (`self.Mesh`) "R_Hand" "KeepRelative" "KeepRelative" "KeepRelative" true))

(fn `Check Left/Right`
  (params (`Spline Rotation` :type "Rotator Structure") (`Degree Range` :type "Float (double-precision)") (`Spline Location` :type "Vector Structure"))
  (returns (`Is Right?` :type Boolean))
  (bind _returnvalue (`KismetMathLibrary.GetRightVector` `Spline Rotation`))
  (bind _returnvalue_2 (`KismetMathLibrary.GetDirectionUnitVector` `Spline Location` (`self.K2_GetActorLocation`)))
  (return (< `Degree Range` (`KismetMathLibrary.DegAcos` (/ (`KismetMathLibrary.Dot_VectorVector` _returnvalue _returnvalue_2) (* (`KismetMathLibrary.VSize` _returnvalue) (`KismetMathLibrary.VSize` _returnvalue_2)))))))

(fn `UserConstructionScript`)