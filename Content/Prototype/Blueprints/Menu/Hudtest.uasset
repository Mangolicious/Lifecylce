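; Hudtest is a prototype mesh-based HUD star bar that shows the BP_Jin player's health and energy.
; Each tick it eases Health and Energy toward the player's current-to-max ratios with FInterpTo, health faster than energy.
; Those values drive a Percent parameter on three material slots: bar and stars for health, a third for energy.
; The dynamic material instances are created in the construction script and recreated every tick rather than cached.
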(event `self.ReceiveTick`
  (params (DeltaSeconds :type "Float (single-precision)"))
  (bind _returnvalue (`GameplayStatics.GetWorldDeltaSeconds`))
  (bind _staticmesh (`self.StaticMesh`))
  (bind _health (`self.Health`))
  (bind _asbp_jin (cast `/Game/Prototype/Blueprints/PlayerCharacter/BP_Jin` (`GameplayStatics.GetPlayerCharacter` 0) :!pure true))
  (set `self.Health` (`KismetMathLibrary.FInterpTo` (`self.Health`) (/ (`/Game/Prototype/Blueprints/PlayerCharacter/BP_Jin.Health` _asbp_jin) (`/Game/Prototype/Blueprints/PlayerCharacter/BP_Jin.Max Health` _asbp_jin)) _returnvalue 2.0))
  (set `self.Energy` (`KismetMathLibrary.FInterpTo` (`self.Energy`) (/ (`/Game/Prototype/Blueprints/PlayerCharacter/BP_Jin.Energy` _asbp_jin) (`/Game/Prototype/Blueprints/PlayerCharacter/BP_Jin.Max Energy` _asbp_jin)) _returnvalue 1.0))
  (bind _returnvalue_2 (`PrimitiveComponent.CreateDynamicMaterialInstance` _staticmesh 0 "/Game/Prototype/Blueprints/Menu/M_Starbar.M_Starbar" "None"))
  (bind _returnvalue_3 (`PrimitiveComponent.CreateDynamicMaterialInstance` _staticmesh 1 "/Game/Prototype/Blueprints/Menu/M_StarbarStars.M_StarbarStars" "None"))
  (bind _returnvalue_4 (`PrimitiveComponent.CreateDynamicMaterialInstance` _staticmesh 2 "/Game/Prototype/Blueprints/Menu/M_StarbarEnergy.M_StarbarEnergy" "None"))
  (`MaterialInstanceDynamic.SetScalarParameterValue` _returnvalue_2 "Percent" _health)
  (`MaterialInstanceDynamic.SetScalarParameterValue` _returnvalue_3 "Percent" _health)
  (`MaterialInstanceDynamic.SetScalarParameterValue` _returnvalue_4 "Percent" (`self.Energy`)))

(fn `UserConstructionScript`
  (bind _staticmesh (`self.StaticMesh`))
  (bind _health (`self.Health`))
  (bind _returnvalue (`PrimitiveComponent.CreateDynamicMaterialInstance` _staticmesh 0 "/Game/Prototype/Blueprints/Menu/M_Starbar.M_Starbar" "None"))
  (bind _returnvalue_2 (`PrimitiveComponent.CreateDynamicMaterialInstance` _staticmesh 1 "/Game/Prototype/Blueprints/Menu/M_StarbarStars.M_StarbarStars" "None"))
  (`MaterialInstanceDynamic.SetScalarParameterValue` _returnvalue "Percent" _health)
  (`MaterialInstanceDynamic.SetScalarParameterValue` _returnvalue_2 "Percent" _health)
  (bind _returnvalue_3 (`PrimitiveComponent.CreateDynamicMaterialInstance` _staticmesh 2 "/Game/Prototype/Blueprints/Menu/M_StarbarEnergy.M_StarbarEnergy" "None"))
  (`MaterialInstanceDynamic.SetScalarParameterValue` _returnvalue_3 "Percent" (`self.Energy`)))