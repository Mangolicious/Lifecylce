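; Ability galaxy menu actor where the player moves a camera between ability nodes and upgrades the selected one with E.
; An intro timeline tilts and zooms the spring-arm camera, then look axes control zoom and yaw.
; Tick sphere-traces along camera-relative movement input to pick the next AbilityComponent, toggling collision on selected nodes.
; Timelines glide the camera root to the selection, or back to center on Evade, with CanSelect gating input meanwhile.
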(event `self.ReceiveBeginPlay`
  (bind _returnvalue (`self.GetController`))
  (bind (_returnvalue_roll _returnvalue_pitch _returnvalue_yaw) (`KismetMathLibrary.BreakRotator` (`Controller.GetControlRotation` _returnvalue)))
  ;[0.2747 0.0137 0.01298] Start
  (`|ExecutionSequence`
    (:`then_0`
      (bind (_direction _lerp_alpha) (`Timeline|CameraStart` :!via `PlayFromStart`)
        (:`Update`
          (`Controller.SetControlRotation` _returnvalue (`KismetMathLibrary.MakeRotator` _returnvalue_roll (`KismetMathLibrary.Lerp` 0.0 -45.0 _lerp_alpha) _returnvalue_yaw))
          (set `SpringArmComponent.TargetArmLength` (`KismetMathLibrary.Lerp` (`self.MinZoom`) (`self.MaxZoom`) _lerp_alpha) (`self.SpringArm`)))))))

(event `InputAxis|LookUp` :overrideparent false
  (params (AxisValue :type "Float (single-precision)"))
  (bind _springarm (`self.SpringArm`))
  ;[0.003035 0.2961 0.6308] Zoom
  (set `SpringArmComponent.TargetArmLength` (`KismetMathLibrary.FClamp` (+ (`SpringArmComponent.TargetArmLength` _springarm) (* AxisValue (`self.Zoomrate`) (`GameplayStatics.GetWorldDeltaSeconds`))) (`self.MinZoom`) (`self.MaxZoom`)) _springarm))

(event `InputAxis|LookUpRate`
  (params (AxisValue :type "Float (single-precision)"))
  (bind _springarm (`self.SpringArm`))
  ;[0.003035 0.2961 0.6308] Zoom
  (set `SpringArmComponent.TargetArmLength` (`KismetMathLibrary.FClamp` (+ (`SpringArmComponent.TargetArmLength` _springarm) (* AxisValue (`self.Zoomrate`) (`GameplayStatics.GetWorldDeltaSeconds`))) (`self.MinZoom`) (`self.MaxZoom`)) _springarm))

(event `Key|E`
  (params (Key :type "Key Structure"))
  ;[1 1 1] Input
  (:`Pressed`
    (`/Game/Prototype/Blueprints/Menu/AbilityComponent.Upgrade Ability` (`self.Selected Ability`))))

(event `InputAxis|TurnRate`
  (params (AxisValue :type "Float (single-precision)"))
  ;[0.3231 0.8963 0.05448] Yaw
  (`self.AddControllerYawInput` AxisValue))

(event `InputAxis|Turn` :overrideparent false
  (params (AxisValue :type "Float (single-precision)"))
  ;[0.3231 0.8963 0.05448] Yaw
  (`self.AddControllerYawInput` AxisValue))

(event `self.ReceiveTick`
  (params (DeltaSeconds :type "Float (single-precision)"))
  (bind _returnvalue (`self.GetInputAxisValue`))
  (bind _returnvalue_2 (`self.GetInputAxisValue`))
  (bind _current_position (`self.Current Position`))
  (bind _selection_deadzone (`self.Selection Deadzone`))
  (bind _returnvalue_3 (* -1 _selection_deadzone))
  (bind (_returnvalue_roll _returnvalue_pitch _returnvalue_yaw) (`KismetMathLibrary.BreakRotator` (`Controller.GetControlRotation` (`self.GetController`))))
  ;[0.9473 0.5583 0.016] Switch Selection
  (if (`self.Can Select?`)
    (if (or (>= _returnvalue _selection_deadzone) (>= _returnvalue _returnvalue_3) (>= _returnvalue_2 _selection_deadzone) (>= _returnvalue_2 _returnvalue_3))
      (bind (_outhit _returnvalue_4) (`KismetSystemLibrary.SphereTraceSingle` :`Start` _current_position :`End` (+ _current_position (* (`KismetMathLibrary.RotateAngleAxis` (`KismetMathLibrary.Normal` (`KismetMathLibrary.MakeVector` (`self.GetInputAxisValue`) (`self.GetInputAxisValue`))) _returnvalue_yaw (0.0 0.0 1.0)) 500.0)) :`Radius` 50.0 :`TraceChannel` "TraceTypeQuery3" :`bIgnoreSelf` false))
      (if _returnvalue_4
        (`/Engine/EditorBlueprintResources/StandardMacros.DoOnce` false :!label _label
          (:`Completed`
            (set `self.Can Select?` false)
            (bind (_bblockinghit _binitialoverlap _time _distance _location _impactpoint _normal _impactnormal _physmat _hitactor _hitcomponent) (`GameplayStatics.BreakHitResult` _outhit))
            (if (!= _hitcomponent (`self.Current Ability`))
              (`PrimitiveComponent.SetCollisionEnabled` (`self.Current Ability`) "QueryAndPhysics")
              (set `self.New Position` (`SceneComponent.K2_GetComponentLocation` _hitcomponent))
              (bind _output_get (set `self.Current Ability` _hitcomponent))
              (bind _asability_component (cast `/Game/Prototype/Blueprints/Menu/AbilityComponent` (`|GetArrayItem` (`SceneComponent.GetParentComponents` _output_get)))
                (:`then`
                  (set `self.Selected Ability` _asability_component)
                  (bind (_direction _lerp_alpha) (`Timeline|Move to Ability` :!via `PlayFromStart` :!label _label_2)
                    (:`Update`
                      (bind _returnvalue_5 (`KismetMathLibrary.VLerp` (`self.Current Position`) (`self.New Position`) _lerp_alpha))
                      (`SceneComponent.K2_SetRelativeLocation` (`self.Camera Root`) _returnvalue_5 false false)
                      (if (== _lerp_alpha 1.0)
                        (set `self.Current Position` _returnvalue_5)
                        (set `self.Can Select?` true)
                        (`PrimitiveComponent.SetCollisionEnabled` _hitcomponent "NoCollision")
                        (`PrimitiveComponent.SetCollisionEnabled` _output_get "NoCollision")
                        (goto _label :!via `Reset`)))))
                (:`CastFailed`
                  (goto _label_2 :!via `PlayFromStart`))))))))))

(event `InputAction|Evade Action`
  (params (Key :type "Key Structure"))
  (bind _returnvalue (`self.K2_GetActorLocation`))
  ;[1 0.4188 0] Reset Selection
  (:`Pressed`
    (if (`self.Can Select?`)
      (set `self.Can Select?` false)
      (`PrimitiveComponent.SetCollisionEnabled` (`self.Current Ability`) "QueryAndPhysics")
      (set `self.Current Ability` null)
      (bind (_direction _lerp_alpha) (`Timeline|Reset to Center` :!via `PlayFromStart`)
        (:`Update`
          (`SceneComponent.K2_SetRelativeLocation` (`self.Camera Root`) (`KismetMathLibrary.VLerp` (`self.Current Position`) _returnvalue _lerp_alpha) false false)
          (if (== _lerp_alpha 1.0)
            (set `self.Current Position` _returnvalue)
            (set `self.Can Select?` true)))))))

(fn `UserConstructionScript`
  (bind _output_get (set `self.Ability Array` (`self.K2_GetComponentsByClass` "/Game/Prototype/Blueprints/Menu/AbilityComponent.AbilityComponent_C")))
  (for _ _output_get
    _))