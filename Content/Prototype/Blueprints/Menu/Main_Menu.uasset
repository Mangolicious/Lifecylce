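; Main menu Blueprint with 3D Play and Quit buttons that open the Blockout level or quit the game.
; Each Tick, a mouse-deprojected line trace positions a cursor, while hover events toggle Highlight on each button's dynamic material.
; Any key enables controller mode through a DoOnce, which Attack re-arms while disabling that mode.
; In controller mode MoveForward moves the highlight, and Jump selects by the axis sign regardless of mode.
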(event `self.ReceiveTick`
  (params (DeltaSeconds :type "Float (single-precision)"))
  (bind (_worldlocation _worlddirection) (`PlayerController.DeprojectMousePositionToWorld` (`GameplayStatics.GetPlayerController` 0)))
  (bind _asmenu_control_bp (cast `/Game/Prototype/Blueprints/Menu/Menu_Control_Bp` (`GameplayStatics.GetPlayerPawn` 0)))
  (bind (_outhit _returnvalue) (`KismetSystemLibrary.LineTraceSingle` _worldlocation (+ _worldlocation (* _worlddirection 800.0)) "TraceTypeQuery2" false (`|MakeArray` _asmenu_control_bp :!type "Actor Object Reference")))
  (bind (_bblockinghit _binitialoverlap _time _distance _location _impactpoint _normal _impactnormal _physmat _hitactor _hitcomponent _hitbonename _hititem _faceindex _tracestart _traceend) (`GameplayStatics.BreakHitResult` _outhit))
  (`SceneComponent.K2_SetWorldLocation` (`self.Cursor`) (select `bool` _returnvalue :`false` _traceend :`true` _location) false false))

(event `self.ReceiveBeginPlay`
  (`KismetSystemLibrary.ResetGamepadAssignmentToController` 0)
  (bind _returnvalue (`PrimitiveComponent.CreateDynamicMaterialInstance` (`self.Play_Button`) 0 "/Game/Prototype/Blueprints/Menu/M_Menu_Inst.M_Menu_Inst" "None"))
  (set `self.Play Instance` _returnvalue)
  (bind _returnvalue_2 (`PrimitiveComponent.CreateDynamicMaterialInstance` (`self.Quit_Button`) 0 "/Game/Prototype/Blueprints/Menu/M_Menu_Inst.M_Menu_Inst" "None"))
  (set `self.Quit Instance` _returnvalue_2))

(event `InputAction|Attack Action`
  (params (Key :type "Key Structure"))
  (:`Pressed`
    (set `self.Controller Active` false)
    (goto _label_3 :!via `Reset`)))

(event `self.Play.OnClicked`
  (params (TouchedComponent :type "PrimitiveComponent Object Reference") (ButtonPressed :type "Key Structure"))
  (`KismetSystemLibrary.PrintString` "Play" :!label _label)
  (`GameplayStatics.OpenLevel` "Blockout"))

(event `self.Play.OnBeginCursorOver`
  (params (TouchedComponent :type "PrimitiveComponent Object Reference"))
  (`MaterialInstanceDynamic.SetScalarParameterValue` (`self.Play Instance`) "Highlight" 1.0 :!label _label_2))

(event `Key|AnyKey`
  (params (Key :type "Key Structure"))
  (:`Pressed`
    (`/Engine/EditorBlueprintResources/StandardMacros.DoOnce` false :!label _label_3
      (:`Completed`
        (set `self.Controller Active` true)))))

(event `self.Play.OnEndCursorOver`
  (params (TouchedComponent :type "PrimitiveComponent Object Reference"))
  (`MaterialInstanceDynamic.SetScalarParameterValue` (`self.Play Instance`) "Highlight" 0.0 :!label _label_4))

(event `InputAxis|MoveForward`
  (params (AxisValue :type "Float (single-precision)"))
  (bind _quit_instance (`self.Quit Instance`))
  (if (`self.Controller Active`)
    (if (>= AxisValue 0.0)
      (`|ExecutionSequence`
        (:`then_0`
          (goto _label_2))
        (:`then_1`
          (`MaterialInstanceDynamic.SetScalarParameterValue` _quit_instance "Highlight" 0.0 :!label _label_5)))
      (else
        (`|ExecutionSequence`
          (:`then_0`
            (`MaterialInstanceDynamic.SetScalarParameterValue` _quit_instance "Highlight" 1.0 :!label _label_6))
          (:`then_1`
            (goto _label_4)))))))

(event `self.Quit.OnClicked`
  (params (TouchedComponent :type "PrimitiveComponent Object Reference") (ButtonPressed :type "Key Structure"))
  (`KismetSystemLibrary.PrintString` "Quit")
  (`KismetSystemLibrary.QuitGame` null "Quit" :!label _label_7))

(event `self.Quit.OnBeginCursorOver`
  (params (TouchedComponent :type "PrimitiveComponent Object Reference"))
  (goto _label_6))

(event `self.Quit.OnEndCursorOver`
  (params (TouchedComponent :type "PrimitiveComponent Object Reference"))
  (goto _label_5))

(event `InputAction|Jump Action`
  (params (Key :type "Key Structure"))
  (:`Pressed`
    (if (>= (stale `InputAxis|MoveForward` AxisValue) 0.0)
      (goto _label)
      (else
        (goto _label_7)))))

(fn `UserConstructionScript`)