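; Menu_Control is a prototype menu Blueprint that moves a world-space Cursor component to follow the mouse.
; On BeginPlay it places the player's mouse at a fixed screen position.
; Each tick it deprojects the mouse, line traces along that ray on the Camera channel with debug drawing, and moves Cursor to the hit point, or to the trace end when nothing is hit.
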(event `self.ReceiveBeginPlay`
  (`PlayerController.SetMouseLocation` (`GameplayStatics.GetPlayerController` 0) 1000 500))

(event `self.ReceiveTick`
  (params (DeltaSeconds :type "Float (single-precision)"))
  (bind (_worldlocation _worlddirection) (`PlayerController.DeprojectMousePositionToWorld` (`GameplayStatics.GetPlayerController` 0)))
  (bind (_outhit _returnvalue) (`KismetSystemLibrary.LineTraceSingle` :`Start` _worldlocation :`End` (+ _worldlocation (* _worlddirection 5000.0)) :`TraceChannel` "TraceTypeQuery2" :`DrawDebugType` "ForOneFrame"))
  (bind (_bblockinghit _binitialoverlap _time _distance _location _impactpoint _normal _impactnormal _physmat _hitactor _hitcomponent _hitbonename _hititem _faceindex _tracestart _traceend) (`GameplayStatics.BreakHitResult` _outhit))
  (`SceneComponent.K2_SetWorldLocation` (`self.Cursor`) (select `bool` _returnvalue :`false` _traceend :`true` _location) false false))

(fn `UserConstructionScript`)