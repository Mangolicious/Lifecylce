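; Shard pickup that grants karma and energy when BP_Jin overlaps its sphere.
; BeginPlay picks a random Moral vector by rotating the X axis around (1,1,1), and construction randomizes the actor's scale.
; On pickup it spawns an explosion, sends KarmaAmount and Moral to Lijar_GameInstance, adds energy to Jin, then destroys itself.
; Mesh variation, impulse and Moral-based particle coloring are disconnected and never run.
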(event `self.ReceiveBeginPlay`
  (set `self.Moral` (`KismetMathLibrary.RotateAngleAxis` (1.0 0.0 0.0) (`KismetMathLibrary.Lerp` 0.0 360.0 (`KismetMathLibrary.RandomFloatInRange` 0.0 1.0)) (1.0 1.0 1.0))))

(event `self.Sphere.OnComponentBeginOverlap`
  (params (OverlappedComponent :type "PrimitiveComponent Object Reference") (OtherActor :type "Actor Object Reference") (OtherComp :type "PrimitiveComponent Object Reference") (OtherBodyIndex :type Integer) (bFromSweep :type Boolean) (SweepResult :type "HitResult Structure (by ref)"))
  (bind _returnvalue (`KismetMathLibrary.Conv_IntToDouble` (`self.Karma Amount`)))
  (bind _asbp_jin (cast `/Game/Prototype/Blueprints/BP_Jin` OtherActor))
  (`GameplayStatics.SpawnEmitterAtLocation` "/Game/Prototype/Particles/Shards/P_ShardExplosion.P_ShardExplosion" (`SceneComponent.K2_GetComponentLocation` (`self.StaticMesh`)))
  (bind _aslijar_game_instance (cast `/Game/Prototype/Blueprints/Lijar_Gameinstance` (`GameplayStatics.GetGameInstance`)))
  (`/Game/Prototype/Blueprints/Lijar_Gameinstance.Karma Update` _aslijar_game_instance _returnvalue (* (`self.Moral`) 1.0))
  (`/Game/Prototype/Blueprints/BP_Jin.Add Energy` _asbp_jin _returnvalue)
  (`self.K2_DestroyActor`))

(fn `UserConstructionScript`
  (`self.SetActorScale3D` (`KismetMathLibrary.Conv_DoubleToVector` (`KismetMathLibrary.RandomFloatInRange` 0.5 1.0))))