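; Blueprint function library of shared helpers for querying the player character, BP_Jin, and its spline movement.
; It reports whether player 0 is dead from its Health, and whether it is on a spline in the air or on a surface, using IsOnSpline and the falling state.
; A further helper estimates an actor's distance along a spline by linearly interpolating between neighboring spline point distances from the closest input key.
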(fn `Get Actor Distance Along Spline`
  (params (`Spline Component` :type "SplineComponent Object Reference") (`Actor World Location` :type "Vector Structure"))
  (returns (`Distance Along Spline` :type "Float (double-precision)"))
  (bind _returnvalue (`SplineComponent.FindInputKeyClosestToWorldLocation` `Spline Component` `Actor World Location`))
  (bind _returnvalue_2 (`KismetMathLibrary.FTrunc` _returnvalue))
  (bind _returnvalue_3 (`SplineComponent.GetDistanceAlongSplineAtSplinePoint` `Spline Component` _returnvalue_2))
  (return (+ _returnvalue_3 (* (- (`SplineComponent.GetDistanceAlongSplineAtSplinePoint` `Spline Component` (`KismetMathLibrary.FTrunc` (+ _returnvalue 1.0))) _returnvalue_3) (- _returnvalue (`KismetMathLibrary.Conv_IntToDouble` _returnvalue_2))))))

(fn `On Spline Mode?`
  (returns (`On Spline Air` :type Boolean) (`On Spline Surface` :type Boolean))
  (bind _asbp_jin (cast `/Game/Prototype/Blueprints/BP_Jin` (`GameplayStatics.GetPlayerCharacter` null) :!pure true))
  (bind _isonspline_ (`/Game/Prototype/Blueprints/BP_Jin.IsOnSpline?` _asbp_jin))
  (bind _returnvalue (`NavMovementComponent.IsFalling` (`Character.CharacterMovement` _asbp_jin)))
  (return (and _isonspline_ _returnvalue) (and _isonspline_ (not _returnvalue))))

(fn `Player Is Dead?`
  (returns (`Is Dead?` :type Boolean))
  (return (<= (`/Game/Prototype/Blueprints/BP_Jin.Health` (cast `/Game/Prototype/Blueprints/BP_Jin` (`GameplayStatics.GetPlayerCharacter` null) :!pure true)) 0.0)))