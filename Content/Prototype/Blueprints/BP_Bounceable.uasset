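; BP_Bounceable is a prototype bounceable actor with a configurable mesh and material, applied to its StaticMesh in the construction script.
; Sphere overlap creates a dynamic material instance on each entry and sets its Color to bright blue, then to a dimmer teal on exit.
; A SpawnVFX event emits BurstEffect at the actor's location; the file contains no bounce logic or caller for that event.
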(event `/Game/Prototype/Blueprints/BPI_SpawnVFX.Spawn VFX`
  (`GameplayStatics.SpawnEmitterAtLocation` (`self.Burst Effect`) (`self.K2_GetActorLocation`)))

(event `self.Sphere.OnComponentBeginOverlap`
  (params (OverlappedComponent :type "PrimitiveComponent Object Reference") (OtherActor :type "Actor Object Reference") (OtherComp :type "PrimitiveComponent Object Reference") (OtherBodyIndex :type Integer) (bFromSweep :type Boolean) (SweepResult :type "HitResult Structure (by ref)"))
  (bind _staticmesh (`self.StaticMesh`))
  (`/Engine/EditorBlueprintResources/StandardMacros.IsValid` OtherActor
    (:`Is Valid`
      (bind _returnvalue (`PrimitiveComponent.CreateDynamicMaterialInstance` _staticmesh 0 (`PrimitiveComponent.GetMaterial` _staticmesh 0) "None"))
      (bind _output_get (set `self.Material Instance` _returnvalue))
      (`MaterialInstanceDynamic.SetVectorParameterValue` _output_get "Color" (struct :`G` 5.755341 :`B` 30.0 :`A` 1.0)))))

(event `self.Sphere.OnComponentEndOverlap`
  (params (OverlappedComponent :type "PrimitiveComponent Object Reference") (OtherActor :type "Actor Object Reference") (OtherComp :type "PrimitiveComponent Object Reference") (OtherBodyIndex :type Integer))
  (`MaterialInstanceDynamic.SetVectorParameterValue` (`self.Material Instance`) "Color" (struct :`G` 2.0 :`B` 1.410965 :`A` 1.0)))

(fn `UserConstructionScript`
  (bind _staticmesh (`self.StaticMesh`))
  (`StaticMeshComponent.SetStaticMesh` _staticmesh (`self.Mesh`))
  (`PrimitiveComponent.SetMaterial` _staticmesh 0 (`self.Material`)))