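; BP_JinProjectile is a prototype player projectile that deals damage and destroys itself on hit.
; Its Hit event prints the object type, then sends direct damage by message to pawns and enemies, or applies radial damage sparing the player for world, destructible and projectile hits.
; A second sequence branch also runs the radial path after every hit.
; Both paths spawn an arrow impact effect scaled by damage.
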(event `self.ReceiveBeginPlay`)

(event `self.ReceiveHit`
  (params (MyComp :type "PrimitiveComponent Object Reference") (Other :type "Actor Object Reference") (OtherComp :type "PrimitiveComponent Object Reference") (bSelfMoved :type Boolean) (HitLocation :type "Vector Structure") (HitNormal :type "Vector Structure") (NormalImpulse :type "Vector Structure") (Hit :type "HitResult Structure (by ref)"))
  (bind _returnvalue (`PrimitiveComponent.GetCollisionObjectType` OtherComp))
  (bind _returnvalue_2 (`self.K2_GetActorLocation`))
  (bind _damage (`self.Damage`))
  (bind _returnvalue_3 (* (1.0 1.0 1.0) (/ (`self.Damage`) 30.0)))
  (`|ExecutionSequence`
    (:`then_0`
      (`KismetSystemLibrary.PrintString` (`|GetEnumeratorNameAsString` _returnvalue))
      (switch `ECollisionChannel` _returnvalue
        (:`ECC_WorldStatic`
          (`GameplayStatics.SpawnEmitterAtLocation` "/Game/Prototype/Particles/Character/WeaponVFX/P_ArrowHitEffect.P_ArrowHitEffect" _returnvalue_2 (struct) _returnvalue_3 :!label _label)
          (`GameplayStatics.ApplyRadialDamage` _damage _returnvalue_2 (`self.Radius`) (`self.Damage Type`) (`|MakeArray` (`GameplayStatics.GetPlayerCharacter` 0) :!type "Actor Object Reference") self null))
        (:`ECC_WorldDynamic`
          (goto _label))
        (:`ECC_Pawn`
          (`GameplayStatics.SpawnEmitterAtLocation` "/Game/Prototype/Particles/Character/WeaponVFX/P_ArrowHitEffect.P_ArrowHitEffect" _returnvalue_2 (struct) _returnvalue_3 :!label _label_2)
          (message `/Game/Prototype/Blueprints/AI/Combat_BPI.Take Damage` Other _damage "None" null Hit))
        (:`ECC_Destructible`
          (goto _label))
        (:`ECC_GameTraceChannel1`
          (goto _label))
        (:`ECC_GameTraceChannel3`
          (goto _label_2))))
    (:`then_1`
      (goto _label)))
  (`self.K2_DestroyActor`))

(fn `UserConstructionScript`)