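; BP_SpiritBlade is a prototype player sword that damages actors overlapping its hitbox while that hitbox is active.
; On overlap it sends a damage message with fixed damage, the hit bone and the player character as causer.
; A short line trace from the blade's Arrow component then finds the impact point to spawn a randomly scaled hit particle, plus a debug print.
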(event `self.Hitbox.OnComponentBeginOverlap`
  (params (OverlappedComponent :type "PrimitiveComponent Object Reference") (OtherActor :type "Actor Object Reference") (OtherComp :type "PrimitiveComponent Object Reference") (OtherBodyIndex :type Integer) (bFromSweep :type Boolean) (SweepResult :type "HitResult Structure (by ref)"))
  (bind _arrow (`self.Arrow`))
  (bind _returnvalue (`SceneComponent.K2_GetComponentLocation` _arrow))
  (if (`self.Hitbox Active?`)
    (message `/Game/Prototype/Blueprints/AI/Combat_BPI.Take Damage` OtherActor 50.0 (`.HitBoneName` (`GameplayStatics.BreakHitResult` SweepResult)) (`GameplayStatics.GetPlayerCharacter` 0) SweepResult)
    (bind (_outhit _returnvalue_2) (`KismetSystemLibrary.LineTraceSingle` _returnvalue (+ (* (`SceneComponent.GetForwardVector` _arrow) 100.0) _returnvalue) "TraceTypeQuery3" true))
    (if _returnvalue_2
      (`GameplayStatics.SpawnEmitterAtLocation` "/Game/Prototype/Particles/P_HitSword.P_HitSword" (`.ImpactPoint` (`GameplayStatics.BreakHitResult` _outhit)) (struct) (`KismetMathLibrary.Conv_DoubleToVector` (`KismetMathLibrary.RandomFloatInRange` 0.7 1.2)))
      (`KismetSystemLibrary.PrintString` "Hit"))))

(fn `UserConstructionScript`)