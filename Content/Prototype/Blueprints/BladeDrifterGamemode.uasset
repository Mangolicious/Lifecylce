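; BladeDrifterGamemode is a game mode that chooses the player's spawn point from respawn state stored in the game instance.
; Its FindPlayerStart function compares each PlayerStart's tag, as a string, to RespawnIndex from Lijar_GameInstance and returns the first match.
; It prints "Error" for every non-matching start it checks, and a separate message if the game instance cast fails.
; BeginPlay only casts the game instance.
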(event `self.ReceiveBeginPlay`
  (bind _aslijar_game_instance (cast `/Game/Prototype/Blueprints/Lijar_Gameinstance` (`GameplayStatics.GetGameInstance`))))

(fn `FindPlayerStart`
  (params (Player :type "Controller Object Reference") (IncomingName :type String))
  (returns (ReturnValue :type "Actor Object Reference"))
  (bind _aslijar_game_instance (cast `/Game/Prototype/Blueprints/Lijar_Gameinstance` (`GameplayStatics.GetGameInstance`))
    (:`then`
      (bind _outactors (`GameplayStatics.GetAllActorsOfClass` "/Script/Engine.PlayerStart"))
      (for _array_element _outactors
        (if (`KismetStringLibrary.EqualEqual_StrStr` (`KismetStringLibrary.Conv_NameToString` (`PlayerStart.PlayerStartTag` _array_element)) (`KismetStringLibrary.Conv_IntToString` (`/Game/Prototype/Blueprints/Lijar_Gameinstance.Respawn Index` _aslijar_game_instance)))
          (return _array_element)
          (else
            (`KismetSystemLibrary.PrintString` "Error")))))
    (:`CastFailed`
      (`KismetSystemLibrary.PrintString` "No Game Instance"))))

(fn `UserConstructionScript`)