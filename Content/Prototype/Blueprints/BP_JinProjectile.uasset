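; BP_JinProjectile is an arrow-effect projectile that plays a spawn emitter and deals damage on impact.
; On hit, it prints and switches on its own hit component's collision type: Pawn and Enemy deal direct damage, others radial damage sparing the player.
; Impact effects scale with Damage, and the actor destroys itself.
; A second Sequence pin repeats the radial-damage branch after every hit.
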(event `self.ReceiveBeginPlay`
  (`GameplayStatics.SpawnEmitterAtLocation` "/Game/Prototype/Particles/Character/WeaponVFX/P_ArrowSpawn.P_ArrowSpawn" (`self.K2_GetActorLocation`) (`self.K2_GetActorRotation`) (2.0 2.0 2.0)))

(event `self.Sphere.OnComponentBeginOverlap`
  (params (OverlappedComponent :type "PrimitiveComponent Object Reference") (OtherActor :type "Actor Object Reference") (OtherComp :type "PrimitiveComponent Object Reference") (OtherBodyIndex :type Integer) (bFromSweep :type Boolean) (SweepResult :type "HitResult Structure (by ref)")))

(event `self.Sphere.OnComponentHit`
  (params (HitComponent :type "PrimitiveComponent Object Reference") (OtherActor :type "Actor Object Reference") (OtherComp :type "PrimitiveComponent Object Reference") (NormalImpulse :type "Vector Structure") (Hit :type "HitResult Structure (by ref)"))
  (bind _returnvalue (`PrimitiveComponent.GetCollisionObjectType` HitComponent))
  (bind _returnvalue_2 (`self.K2_GetActorLocation`))
  (bind _damage (`self.Damage`))
  (bind _damage_type (`self.Damage Type`))
  (bind _returnvalue_3 (* (1.0 1.0 1.0) (/ (`self.Damage`) 30.0)))
  (`|ExecutionSequence`
    (:`then_0`
      (`KismetSystemLibrary.PrintString` (`|GetEnumeratorNameAsString` _returnvalue))
      (switch `ECollisionChannel` _returnvalue
        (:`ECC_WorldStatic`
          (`GameplayStatics.SpawnEmitterAtLocation` "/Game/Prototype/Particles/Character/WeaponVFX/P_ArrowHitEffect.P_ArrowHitEffect" _returnvalue_2 (struct) _returnvalue_3 :!label _label)
          (`GameplayStatics.ApplyRadialDamage` _damage _returnvalue_2 (`self.Radius`) _damage_type (`|MakeArray` (`GameplayStatics.GetPlayerCharacter` 0) :!type "Actor Object Reference") self null))
        (:`ECC_WorldDynamic`
          (goto _label))
        (:`ECC_Pawn`
          (`GameplayStatics.SpawnEmitterAtLocation` "/Game/Prototype/Particles/Character/WeaponVFX/P_ArrowHitEffect.P_ArrowHitEffect" _returnvalue_2 (struct) _returnvalue_3 :!label _label_2)
          (`GameplayStatics.ApplyDamage` OtherActor _damage null self _damage_type))
        (:`ECC_Destructible`
          (goto _label))
        (:`ECC_GameTraceChannel1`
          (goto _label))
        (:`ECC_GameTraceChannel3`
          (goto _label_2))))
    (:`then_1`
      (goto _label)))
  (`self.K2_DestroyActor`))

(fn `UserConstructionScript`)