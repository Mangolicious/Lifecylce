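; LifeLine spline actor that draws a colored line in the level and boosts BP_Jin's LineSpeed when HitSpline fires.
; The construction script optionally snaps points to the ground with downward traces, then builds spline meshes, pinching and flagging the end segments through material parameters.
; HitSpline also activates a particle system, which Tick keeps slightly ahead of the player's closest spline point by interpolating input key into distance.
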(event `Hit Spline`
  (bind _asbp_jin (cast `/Game/Prototype/Blueprints/BP_Jin` (`GameplayStatics.GetPlayerCharacter` 0)))
  (set `/Game/Prototype/Blueprints/BP_Jin.LineSpeed` (+ (`self.Speed Boost`) (`/Game/Prototype/Blueprints/BP_Jin.LineSpeed` _asbp_jin)) _asbp_jin)
  (`ActorComponent.SetActive` (`self.ParticleSystem`) true false))

(event `self.ReceiveTick`
  (params (DeltaSeconds :type "Float (single-precision)"))
  (bind _spline (`self.Spline`))
  (bind _spline_2 (`self.Spline`))
  (bind _returnvalue (`SplineComponent.FindInputKeyClosestToWorldLocation` _spline (`SceneComponent.K2_GetComponentLocation` (`Character.CapsuleComponent` (`GameplayStatics.GetPlayerCharacter` 0)))))
  (bind _returnvalue_2 (`KismetMathLibrary.FTrunc` _returnvalue))
  (bind _returnvalue_3 (`SplineComponent.GetDistanceAlongSplineAtSplinePoint` _spline_2 _returnvalue_2))
  (bind _returnvalue_4 (+ (+ _returnvalue_3 (* (- (`SplineComponent.GetDistanceAlongSplineAtSplinePoint` _spline (`KismetMathLibrary.FTrunc` (+ _returnvalue 1.0))) _returnvalue_3) (- _returnvalue (`KismetMathLibrary.Conv_IntToDouble` _returnvalue_2)))) 50.0))
  (`SceneComponent.K2_SetWorldLocationAndRotation` (`self.ParticleSystem`) (`SplineComponent.GetLocationAtDistanceAlongSpline` _spline_2 _returnvalue_4 "World") (`SplineComponent.GetRotationAtDistanceAlongSpline` _spline_2 _returnvalue_4 "World") false false))

(fn `UserConstructionScript`
  (bind _spline (`self.Spline`))
  (bind _spline_2 (`self.Spline`))
  (bind _spline_3 (`self.Spline`))
  (bind _scale (`self.Scale`))
  (bind _scale_2 (`self.Scale`))
  (bind _spline_4 (`self.Spline`))
  (bind (_location _tangent) (`SplineComponent.GetLocationAndTangentAtSplinePoint` _spline_3 0 "Local"))
  (bind (_location_2 _tangent_2) (`SplineComponent.GetLocationAndTangentAtSplinePoint` _spline_3 1 "Local"))
  (bind _returnvalue (* _scale_2 (`self.Start End Pinch`)))
  (bind _returnvalue_2 (`SplineComponent.GetNumberOfSplinePoints` _spline_2))
  (bind (_location_3 _tangent_3) (`SplineComponent.GetLocationAndTangentAtSplinePoint` _spline_2 _returnvalue_2 "Local"))
  (bind (_location_4 _tangent_4) (`SplineComponent.GetLocationAndTangentAtSplinePoint` _spline_2 (- _returnvalue_2 2) "Local"))
  (`|ExecutionSequence`
    (:`then_0`
      (if (`self.Trace for Ground?`)
        ;[0.2918 0 0] Trace for Ground
        (for _index (range (+ (`SplineComponent.GetNumberOfSplinePoints` _spline_4) 1))
          (bind _location_5 (`SplineComponent.GetLocationAndTangentAtSplinePoint` _spline_4 _index "World"))
          (bind (_outhit _returnvalue_3) (`KismetSystemLibrary.LineTraceSingle` :`Start` _location_5 :`End` (+ _location_5 (0.0 0.0 -500.0)) :`TraceChannel` "TraceTypeQuery1" :`DrawDebugType` "ForDuration"))
          (if _returnvalue_3
            (`SplineComponent.SetLocationAtSplinePoint` (`self.Spline`) _index (+ (`.Location` (`GameplayStatics.BreakHitResult` _outhit)) (`KismetMathLibrary.MakeVector` 0.0 0.0 (`self.Z Offset`))) "World" true)))
        (`SplineComponent.UpdateSpline` (`self.Spline`))))
    (:`then_1`
      (for _index_2 (range 1 (+ (- (`SplineComponent.GetNumberOfSplinePoints` _spline) 3) 1))
        (bind _returnvalue_4 (`AddComponent|NODE_AddSplineMeshComponent-0`))
        (`StaticMeshComponent.SetStaticMesh` _returnvalue_4 (`self.Line Mesh`))
        (`MeshComponent.SetVectorParameterValueOnMaterials` _returnvalue_4 "Color" (`KismetMathLibrary.Conv_LinearColorToVector` (`self.Color`)))
        (bind (_location_6 _tangent_5) (`SplineComponent.GetLocationAndTangentAtSplinePoint` _spline _index_2 "Local"))
        (bind (_location_7 _tangent_6) (`SplineComponent.GetLocationAndTangentAtSplinePoint` _spline (+ _index_2 1) "Local"))
        (`SplineMeshComponent.SetStartAndEnd` _returnvalue_4 _location_6 _tangent_5 _location_7 _tangent_6 true)
        (`SplineMeshComponent.SetStartScale` _returnvalue_4 _scale true)
        (`SplineMeshComponent.SetEndScale` _returnvalue_4 _scale true))
      (`|ExecutionSequence`
        (:`then_0`
          ;[0 0.9671 1] Start
          (bind _returnvalue_5 (`AddComponent|NODE_AddSplineMeshComponent-3`))
          (`StaticMeshComponent.SetStaticMesh` _returnvalue_5 (`self.Line Mesh`))
          (`MeshComponent.SetVectorParameterValueOnMaterials` _returnvalue_5 "Color" (`KismetMathLibrary.Conv_LinearColorToVector` (`self.Color`)))
          (`MeshComponent.SetScalarParameterValueOnMaterials` _returnvalue_5 "Start / End" 0.0)
          (`MeshComponent.SetScalarParameterValueOnMaterials` _returnvalue_5 "Switch" 0.0)
          (`SplineMeshComponent.SetStartAndEnd` _returnvalue_5 _location _tangent _location_2 _tangent_2 true)
          (`SplineMeshComponent.SetStartScale` _returnvalue_5 _returnvalue true)
          (`SplineMeshComponent.SetEndScale` _returnvalue_5 _scale_2 true))
        (:`then_1`
          ;[0 1 0.09921] End
          (bind _returnvalue_6 (`AddComponent|NODE_AddSplineMeshComponent-4`))
          (`StaticMeshComponent.SetStaticMesh` _returnvalue_6 (`self.Line Mesh`))
          (`MeshComponent.SetVectorParameterValueOnMaterials` _returnvalue_6 "Color" (`KismetMathLibrary.Conv_LinearColorToVector` (`self.Color`)))
          (`MeshComponent.SetScalarParameterValueOnMaterials` _returnvalue_6 "Start / End" 1.0)
          (`MeshComponent.SetScalarParameterValueOnMaterials` _returnvalue_6 "Switch" 0.0)
          (`SplineMeshComponent.SetStartAndEnd` _returnvalue_6 _location_4 _tangent_4 _location_3 _tangent_3 true)
          (`SplineMeshComponent.SetEndScale` _returnvalue_6 _returnvalue true)
          (`SplineMeshComponent.SetStartScale` _returnvalue_6 _scale_2 true))))))