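; Scene component that makes its owning actor hover over surfaces using physics forces.
; On BeginPlay it takes the owner's first primitive component, enables physics simulation and applies linear and angular damping.
; Each tick it traces downward, pushing along the hit normal with force fading linearly to zero at trace length.
; A flag selects force at the component's location or a mass-independent acceleration on the body.
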(event `self.ReceiveBeginPlay`
  (bind _output_get (set `self.PrimitiveComponent` (`|GetArrayItem` (`Actor.K2_GetComponentsByClass` (`self.GetOwner`) "/Script/Engine.PrimitiveComponent"))))
  (`PrimitiveComponent.SetSimulatePhysics` _output_get true)
  (`PrimitiveComponent.SetLinearDamping` _output_get (`self.LinearDampening`))
  (`PrimitiveComponent.SetAngularDamping` _output_get (`self.AngularDampening`)))

(event `self.ReceiveTick`
  (params (DeltaSeconds :type "Float (single-precision)"))
  (bind _returnvalue (`self.K2_GetComponentLocation`))
  (bind _primitivecomponent (`self.PrimitiveComponent`))
  (bind (_outhit _returnvalue_2) (`KismetSystemLibrary.LineTraceSingle` _returnvalue (- _returnvalue (`KismetMathLibrary.MakeVector` 0.0 0.0 (`self.TraceLength`))) "TraceTypeQuery1" true))
  (if _returnvalue_2
    (if (`self.UseHoveLocation?`)
      (bind (_bblockinghit _binitialoverlap _time _distance _location _impactpoint _normal _impactnormal) (`GameplayStatics.BreakHitResult` _outhit))
      (bind _returnvalue_3 (* _impactnormal (`KismetMathLibrary.Lerp` (`self.HoverForce`) 0.0 (/ (`KismetMathLibrary.VSize` (- _location (`self.K2_GetComponentLocation`))) (`self.TraceLength`)))))
      (`PrimitiveComponent.AddForceAtLocation` _primitivecomponent _returnvalue_3 (`self.K2_GetComponentLocation`) "None")
      (else
        (`PrimitiveComponent.AddForce` _primitivecomponent _returnvalue_3 "None" true)))))