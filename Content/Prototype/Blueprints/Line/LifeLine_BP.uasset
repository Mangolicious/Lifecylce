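; LifeLine_BP is a spline line that rewards BP_Jin with karma and energy while riding it.
; When toggled active, Tick drains line energy on surface contact, scaling rewards by player speed and karma also by remaining energy.
; Leaving the spline deactivates it after a delay.
; Construction builds colored spline meshes with pinched ends unless ExtraMesh is set, plus debug axis arrows; ground-snapping logic is disconnected.
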(event `Hit Spline Toggle`
  (`/Engine/EditorBlueprintResources/StandardMacros.FlipFlop`
    (:`A`
      (set `self.Active Spline` true))
    (:`B`
      (set `self.Active Spline` false))))

(event `self.ReceiveBeginPlay`
  (set `self.Lifeline Energy` (`self.Max Lifeline Energy`)))

(event `self.ReceiveTick`
  (params (DeltaSeconds :type "Float (single-precision)"))
  (bind (_on_spline_air _on_spline_surface) (`/Game/Prototype/Blueprints/LijarFunctionLibrary.On Spline Mode?`))
  (bind _max_lifeline_energy (`self.Max Lifeline Energy`))
  (if (`self.Active Spline`)
    (bind _asbp_jin (cast `/Game/Prototype/Blueprints/BP_Jin` (`GameplayStatics.GetPlayerCharacter` 0)))
    (if _on_spline_air
      ;[0.1736 0.4896 0.0294] Karma System
      (if _on_spline_surface
        (`KismetSystemLibrary.Delay` (`self.Gain Speed`))
        (bind _aslijar_game_instance (cast `/Game/Prototype/Blueprints/Lijar_Gameinstance` (`GameplayStatics.GetGameInstance`)))
        (bind _returnvalue (/ (`KismetMathLibrary.FClamp` (`KismetMathLibrary.VSize` (`self.GetVelocity` _asbp_jin)) 0.0 4000.0) 4000.0))
        (set `self.Gain Speed` (`KismetMathLibrary.Lerp` 0.1 0.05 _returnvalue))
        (set `self.Lifeline Energy` (`KismetMathLibrary.FClamp` (- (`self.Lifeline Energy`) 1.0) 0.0 (`self.Max Lifeline Energy`)))
        (bind _returnvalue_2 (`KismetMathLibrary.Lerp` 1.0 10.0 _returnvalue))
        (`/Game/Prototype/Blueprints/Lijar_Gameinstance.Karma Update` _aslijar_game_instance (* (`KismetMathLibrary.Lerp` 0.0 (`self.Lifeline Karma Gain`) (/ (`KismetMathLibrary.FClamp` (`self.Lifeline Energy`) 0.0 _max_lifeline_energy) _max_lifeline_energy)) _returnvalue_2) (0.0 0.0 0.0))
        (`/Game/Prototype/Blueprints/BP_Jin.Add Energy` _asbp_jin (* (`self.Lifeline Karma Gain`) _returnvalue_2)))
      (else
        (`KismetSystemLibrary.Delay` 3.0)
        (set `self.Active Spline` false)))))

(fn `Debug Spline Vector`
  (params (Spline :type "SplineComponent Object Reference"))
  (for _index (range (`SplineComponent.GetNumberOfSplinePoints` Spline))
    (`SplineComponent.SetUpVectorAtSplinePoint` Spline _index (`SplineComponent.GetUpVectorAtSplinePoint` Spline _index "Local") "Local" true)
    (bind _returnvalue (`SplineComponent.GetLocationAtSplinePoint` Spline _index "Local"))
    (bind _returnvalue_2 (`SplineComponent.GetUpVectorAtSplinePoint` Spline _index "Local"))
    (bind _returnvalue_3 (`AddComponent|NODE_AddArrowComponent-1` :`RelativeTransform` (`KismetMathLibrary.MakeTransform` _returnvalue (`KismetMathLibrary.Conv_VectorToRotator` _returnvalue_2))))
    (`ArrowComponent.SetArrowColor` _returnvalue_3 (struct :`B` 1.0 :`A` 1.0))
    (bind _returnvalue_4 (`SplineComponent.GetRightVectorAtSplinePoint` Spline _index "Local"))
    (bind _returnvalue_5 (`AddComponent|NODE_AddArrowComponent-2` :`RelativeTransform` (`KismetMathLibrary.MakeTransform` _returnvalue (`KismetMathLibrary.Conv_VectorToRotator` _returnvalue_4))))
    (`ArrowComponent.SetArrowColor` _returnvalue_5 (struct :`G` 1.0 :`A` 1.0))
    (bind _returnvalue_6 (`AddComponent|NODE_AddArrowComponent-3` :`RelativeTransform` (`KismetMathLibrary.MakeTransform` _returnvalue (`KismetMathLibrary.Conv_VectorToRotator` (* (`KismetMathLibrary.Cross_VectorVector` _returnvalue_2 _returnvalue_4) -1)))))
    (`ArrowComponent.SetArrowColor` _returnvalue_6 (struct :`R` 1.0 :`A` 1.0))))

(fn `NewFunction_0`)

(fn `UserConstructionScript`
  (bind _spline (`self.Spline`))
  (bind _spline_2 (`self.Spline`))
  (bind _spline_3 (`self.Spline`))
  (bind _spline_4 (`self.Spline`))
  (bind _spline_5 (`self.Spline`))
  (bind _scale (`self.Scale`))
  (bind _spline_6 (`self.Spline`))
  (bind _scale_2 (`self.Scale`))
  (bind (_location _tangent) (`SplineComponent.GetLocationAndTangentAtSplinePoint` _spline_4 1 "Local"))
  (bind (_location_2 _tangent_2) (`SplineComponent.GetLocationAndTangentAtSplinePoint` _spline_4 0 "Local"))
  (bind _returnvalue (* _scale_2 (`self.Start End Pinch`)))
  (bind _returnvalue_2 (`SplineComponent.GetNumberOfSplinePoints` _spline_3))
  (bind _returnvalue_3 (- _returnvalue_2 2))
  (bind (_location_3 _tangent_3) (`SplineComponent.GetLocationAndTangentAtSplinePoint` _spline_3 _returnvalue_2 "Local"))
  (bind (_location_4 _tangent_4) (`SplineComponent.GetLocationAndTangentAtSplinePoint` _spline_3 _returnvalue_3 "Local"))
  (`self.Debug Spline Vector` _spline)
  (`|ExecutionSequence`
    (:`then_0`
      (if (not (`self.Extra Mesh`))
        (for _index (range 1 (+ (- (`SplineComponent.GetNumberOfSplinePoints` _spline) 3) 1))
          (bind _returnvalue_4 (`AddComponent|NODE_AddSplineMeshComponent-0`))
          (`StaticMeshComponent.SetStaticMesh` _returnvalue_4 (`self.Line Mesh`))
          (`MeshComponent.SetVectorParameterValueOnMaterials` _returnvalue_4 "Color" (`KismetMathLibrary.Conv_LinearColorToVector` (`self.Color`)))
          (bind (_location_5 _tangent_5) (`SplineComponent.GetLocationAndTangentAtSplinePoint` _spline _index "Local"))
          (bind (_location_6 _tangent_6) (`SplineComponent.GetLocationAndTangentAtSplinePoint` _spline (+ _index 1) "Local"))
          (`SplineMeshComponent.SetStartAndEnd` _returnvalue_4 _location_5 _tangent_5 _location_6 _tangent_6 true)
          (`SplineMeshComponent.SetStartScale` _returnvalue_4 _scale true)
          (`SplineMeshComponent.SetEndScale` _returnvalue_4 _scale true)
          (`SplineMeshComponent.SetStartRoll` _returnvalue_4 (`KismetMathLibrary.DegreesToRadians` (.roll (`SplineComponent.GetRotationAtSplinePoint` _spline_2 _index "Local"))) true)
          (`SplineMeshComponent.SetEndRoll` _returnvalue_4 (`KismetMathLibrary.DegreesToRadians` (.roll (`SplineComponent.GetRotationAtSplinePoint` _spline_2 (+ _index 1) "Local"))) true))
        (`|ExecutionSequence`
          (:`then_0`
            ;[0 0.9671 1] Start
            (bind _returnvalue_5 (`AddComponent|NODE_AddSplineMeshComponent-3`))
            (`StaticMeshComponent.SetStaticMesh` _returnvalue_5 (`self.Line Mesh`))
            (`MeshComponent.SetVectorParameterValueOnMaterials` _returnvalue_5 "Color" (`KismetMathLibrary.Conv_LinearColorToVector` (`self.Color`)))
            (`MeshComponent.SetScalarParameterValueOnMaterials` _returnvalue_5 "Start / End" 0.0)
            (`MeshComponent.SetScalarParameterValueOnMaterials` _returnvalue_5 "Switch" 0.0)
            (`SplineMeshComponent.SetStartAndEnd` _returnvalue_5 _location_2 _tangent_2 _location _tangent true)
            (`SplineMeshComponent.SetStartScale` _returnvalue_5 _returnvalue true)
            (`SplineMeshComponent.SetEndScale` _returnvalue_5 _scale_2 true)
            (`SplineMeshComponent.SetStartRoll` _returnvalue_5 (`KismetMathLibrary.DegreesToRadians` (.roll (`SplineComponent.GetRotationAtSplinePoint` _spline_6 0 "Local"))) true)
            (`SplineMeshComponent.SetEndRoll` _returnvalue_5 (`KismetMathLibrary.DegreesToRadians` (.roll (`SplineComponent.GetRotationAtSplinePoint` _spline_6 1 "Local"))) true))
          (:`then_1`
            ;[0 1 0.09921] End
            (bind _returnvalue_6 (`AddComponent|NODE_AddSplineMeshComponent-4`))
            (`StaticMeshComponent.SetStaticMesh` _returnvalue_6 (`self.Line Mesh`))
            (`MeshComponent.SetVectorParameterValueOnMaterials` _returnvalue_6 "Color" (`KismetMathLibrary.Conv_LinearColorToVector` (`self.Color`)))
            (`MeshComponent.SetScalarParameterValueOnMaterials` _returnvalue_6 "Start / End" 1.0)
            (`MeshComponent.SetScalarParameterValueOnMaterials` _returnvalue_6 "Switch" 0.0)
            (`SplineMeshComponent.SetStartAndEnd` _returnvalue_6 _location_4 _tangent_4 _location_3 _tangent_3 true)
            (`SplineMeshComponent.SetEndScale` _returnvalue_6 _returnvalue true)
            (`SplineMeshComponent.SetStartScale` _returnvalue_6 _scale_2 true)
            (`SplineMeshComponent.SetStartRoll` _returnvalue_6 (`KismetMathLibrary.DegreesToRadians` (.roll (`SplineComponent.GetRotationAtSplinePoint` _spline_5 _returnvalue_3 "Local"))) true)
            (`SplineMeshComponent.SetEndRoll` _returnvalue_6 (`KismetMathLibrary.DegreesToRadians` (.roll (`SplineComponent.GetRotationAtSplinePoint` _spline_5 _returnvalue_2 "Local"))) true)))))
    (:`then_2`
      (`ParticleSystemComponent.SetColorParameter` (`self.Line Particle`) "LineColor" (* (`self.Color`) 0.0)))
    (:`then_4`
      (if (not (`self.Extra Mesh`))
        (`ActorComponent.K2_DestroyComponent` (`self.StaticMesh`))))))