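; LineSpline is a spline actor that draws a colored line and moves a sphere along it relative to the player.
; The construction script adds a spline mesh for each segment, using the Line mesh tinted by Color.
; Each tick it converts the spline input key closest to the player's capsule into an interpolated distance, then places and orients the sphere 50 units farther along.
; A random mesh and color variant is left unconnected.
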(event `self.ReceiveTick`
  (params (DeltaSeconds :type "Float (single-precision)"))
  (bind _spline (`self.Spline`))
  (bind _spline_2 (`self.Spline`))
  (bind _returnvalue (`SplineComponent.FindInputKeyClosestToWorldLocation` _spline (`SceneComponent.K2_GetComponentLocation` (`Character.CapsuleComponent` (`GameplayStatics.GetPlayerCharacter` 0)))))
  (bind _returnvalue_2 (`KismetMathLibrary.FTrunc` _returnvalue))
  (bind _returnvalue_3 (`SplineComponent.GetDistanceAlongSplineAtSplinePoint` _spline_2 _returnvalue_2))
  (bind _returnvalue_4 (+ (+ _returnvalue_3 (* (- (`SplineComponent.GetDistanceAlongSplineAtSplinePoint` _spline (`KismetMathLibrary.FTrunc` (+ _returnvalue 1.0))) _returnvalue_3) (- _returnvalue (`KismetMathLibrary.Conv_IntToDouble` _returnvalue_2)))) 50.0))
  (`SceneComponent.K2_SetWorldLocationAndRotation` (`self.Sphere`) (`SplineComponent.GetLocationAtDistanceAlongSpline` _spline_2 _returnvalue_4 "World") (`SplineComponent.GetRotationAtDistanceAlongSpline` _spline_2 _returnvalue_4 "World") false false))

(fn `UserConstructionScript`
  (bind _spline (`self.Spline`))
  (for _index (range (+ (- (`SplineComponent.GetNumberOfSplinePoints` _spline) 2) 1))
    (`|ExecutionSequence`
      (:`then_0`
        (bind _returnvalue (`AddComponent|NODE_AddSplineMeshComponent-0`))
        (`StaticMeshComponent.SetStaticMesh` _returnvalue "/Game/Prototype/Meshes/Line.Line")
        (`MeshComponent.SetVectorParameterValueOnMaterials` _returnvalue "Color" (`KismetMathLibrary.Conv_LinearColorToVector` (`self.Color`)))
        (bind (_location _tangent) (`SplineComponent.GetLocationAndTangentAtSplinePoint` _spline _index "Local"))
        (bind (_location_2 _tangent_2) (`SplineComponent.GetLocationAndTangentAtSplinePoint` _spline (+ _index 1) "Local"))
        (`SplineMeshComponent.SetStartAndEnd` _returnvalue _location _tangent _location_2 _tangent_2 true)))))