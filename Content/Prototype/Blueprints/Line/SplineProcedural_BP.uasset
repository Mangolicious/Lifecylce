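; Prototype procedural spline actor that spawns a lifeline following one of two parallel spline paths.
; The construction script rebuilds SplineSide as a sideways-offset copy of SplineMid, matching point types and tangents.
; BeginPlay spawns a LifeLineTest_BP, adds points, fits it to a randomly picked spline with a slight offset via AddLifelineToSpline, then calls GenerateSpline.
; Unwired leftovers hold earlier point-array, arrow-component and LifeLine_BP experiments.
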(event `self.ReceiveBeginPlay`
  (bind _returnvalue (`|SpawnActorFromClass` "/Game/Prototype/Blueprints/Line/LifeLineTest_BP.LifeLineTest_BP_C" (`KismetMathLibrary.MakeTransform` (`self.K2_GetActorLocation`) (`self.K2_GetActorRotation`)) "AlwaysSpawn" "OverrideRootScale" null null))
  (for _ (range (+ (`self.Number of points`) 1))
    (bind _lifeline_spline (`/Game/Prototype/Blueprints/Line/LifeLineTest_BP.Lifeline Spline` _returnvalue))
    (`SplineComponent.AddSplinePoint` _lifeline_spline (`self.K2_GetActorLocation` _returnvalue) "Local" true))
  (`self.Add Lifeline to Spline` _lifeline_spline (select `int` (`KismetMathLibrary.RandomIntegerInRange` 0 1) :`0` (`self.Spline Mid`) :`1` (`self.Spline Side`)))
  (`/Game/Prototype/Blueprints/Line/LifeLineTest_BP.Generate Spline` _returnvalue)
  (`SplineComponent.UpdateSpline` _lifeline_spline))

(fn `Add Lifeline to Spline`
  (params (`New Spline` :type "SplineComponent Object Reference") (`Attach Spline` :type "SplineComponent Object Reference"))
  (for _index (range (`SplineComponent.GetNumberOfSplinePoints` `New Spline`))
    (bind (_location _tangent) (`SplineComponent.GetLocationAndTangentAtSplinePoint` `Attach Spline` _index "Local"))
    (`SplineComponent.SetLocationAtSplinePoint` `New Spline` _index (+ _location (+ (* (`SplineComponent.GetUpVectorAtSplinePoint` `Attach Spline` _index "Local") 10.0) (* (`SplineComponent.GetRightVectorAtSplinePoint` `Attach Spline` _index "Local") 1.0) (* (`SceneComponent.GetForwardVector` `Attach Spline`) 1.0))) "Local" true)
    (`SplineComponent.SetSplinePointType` `New Spline` _index (`SplineComponent.GetSplinePointType` `Attach Spline` _index) true)
    (`SplineComponent.SetTangentAtSplinePoint` `New Spline` _index _tangent "Local" true)))

(fn `UserConstructionScript`
  (bind _spline_side (`self.Spline Side`))
  (bind _spline_mid (`self.Spline Mid`))
  (`|ExecutionSequence`
    (:`then_0`
      (`SplineComponent.ClearSplinePoints` (`self.Spline Side`) true)
      (for _index (range (`SplineComponent.GetNumberOfSplinePoints` _spline_mid))
        (bind (_location _tangent) (`SplineComponent.GetLocationAndTangentAtSplinePoint` _spline_mid _index "Local"))
        (`SplineComponent.AddSplinePoint` _spline_side (+ _location (+ (* (`SplineComponent.GetUpVectorAtSplinePoint` _spline_mid _index "Local") 0.0) (* (`SplineComponent.GetRightVectorAtSplinePoint` _spline_mid _index "Local") 100.0) (* (`SceneComponent.GetForwardVector` _spline_mid) 1.0))) "Local" true)
        (`SplineComponent.SetSplinePointType` _spline_side _index (`SplineComponent.GetSplinePointType` _spline_mid _index) true)
        (`SplineComponent.SetTangentAtSplinePoint` _spline_side _index _tangent "Local" true)))))