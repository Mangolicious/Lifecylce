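; Prototype lifeline that sets BP_Jin's line speed when hit and rewards riding it.
; Construction snaps it to a nearby OriantationSpline point, copies the remaining points with an offset, and builds colored spline meshes with pinched ends.
; GenerateSpline refills line energy, adds the meshes again and brightens the particle color.
; While ridden, Tick drains line energy, granting speed-scaled player energy and karma that fades with depletion, and deactivates after a delay off-spline.
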(event `Generate Spline`
  (bind _lifeline_spline (`self.Lifeline Spline`))
  (bind _lifeline_spline_2 (`self.Lifeline Spline`))
  (bind _lifeline_spline_3 (`self.Lifeline Spline`))
  (bind _lifeline_spline_4 (`self.Lifeline Spline`))
  (bind _lifeline_spline_5 (`self.Lifeline Spline`))
  (bind _scale (`self.Scale`))
  (bind _scale_2 (`self.Scale`))
  (bind _lifeline_spline_6 (`self.Lifeline Spline`))
  (bind (_location _tangent) (`SplineComponent.GetLocationAndTangentAtSplinePoint` _lifeline_spline_4 0 "Local"))
  (bind (_location_2 _tangent_2) (`SplineComponent.GetLocationAndTangentAtSplinePoint` _lifeline_spline_4 1 "Local"))
  (bind _returnvalue (* _scale_2 (`self.Start End Pinch`)))
  (bind _returnvalue_2 (`SplineComponent.GetNumberOfSplinePoints` _lifeline_spline_2))
  (bind _returnvalue_3 (- _returnvalue_2 2))
  (bind (_location_3 _tangent_3) (`SplineComponent.GetLocationAndTangentAtSplinePoint` _lifeline_spline_2 _returnvalue_2 "Local"))
  (bind (_location_4 _tangent_4) (`SplineComponent.GetLocationAndTangentAtSplinePoint` _lifeline_spline_2 _returnvalue_3 "Local"))
  (set `self.Lifeline Energy` (`self.Max Lifeline Energy`))
  (`|ExecutionSequence`
    (:`then_0`
      (for _index (range 1 (+ (- (`SplineComponent.GetNumberOfSplinePoints` _lifeline_spline) 3) 1))
        (bind _returnvalue_4 (`AddComponent|NODE_AddSplineMeshComponent-5`))
        (`StaticMeshComponent.SetStaticMesh` _returnvalue_4 (`self.Line Mesh`))
        (`MeshComponent.SetVectorParameterValueOnMaterials` _returnvalue_4 "Color" (`KismetMathLibrary.Conv_LinearColorToVector` (`self.Color`)))
        (bind (_location_5 _tangent_5) (`SplineComponent.GetLocationAndTangentAtSplinePoint` _lifeline_spline _index "Local"))
        (bind _returnvalue_5 (+ _index 1))
        (bind (_location_6 _tangent_6) (`SplineComponent.GetLocationAndTangentAtSplinePoint` _lifeline_spline _returnvalue_5 "Local"))
        (`SplineMeshComponent.SetStartAndEnd` _returnvalue_4 _location_5 _tangent_5 _location_6 _tangent_6 true)
        (`SplineMeshComponent.SetStartScale` _returnvalue_4 _scale true)
        (`SplineMeshComponent.SetEndScale` _returnvalue_4 _scale true)
        (`SplineMeshComponent.SetStartRoll` _returnvalue_4 (/ (`SplineComponent.GetRollAtSplinePoint` _lifeline_spline_3 _index "World") 90.0) true)
        (`SplineMeshComponent.SetEndRoll` _returnvalue_4 (/ (`SplineComponent.GetRollAtSplinePoint` _lifeline_spline_3 _returnvalue_5 "World") 90.0) true))
      (`|ExecutionSequence`
        (:`then_0`
          ;[0 0.9671 1] Start
          (bind _returnvalue_6 (`AddComponent|NODE_AddSplineMeshComponent-6`))
          (`StaticMeshComponent.SetStaticMesh` _returnvalue_6 (`self.Line Mesh`))
          (`MeshComponent.SetVectorParameterValueOnMaterials` _returnvalue_6 "Color" (`KismetMathLibrary.Conv_LinearColorToVector` (`self.Color`)))
          (`MeshComponent.SetScalarParameterValueOnMaterials` _returnvalue_6 "Start / End" 0.0)
          (`MeshComponent.SetScalarParameterValueOnMaterials` _returnvalue_6 "Switch" 0.0)
          (`SplineMeshComponent.SetStartAndEnd` _returnvalue_6 _location _tangent _location_2 _tangent_2 true)
          (`SplineMeshComponent.SetStartScale` _returnvalue_6 _returnvalue true)
          (`SplineMeshComponent.SetEndScale` _returnvalue_6 _scale_2 true)
          (`SplineMeshComponent.SetStartRoll` _returnvalue_6 (/ (`SplineComponent.GetRollAtSplinePoint` _lifeline_spline_6 0 "World") 90.0) true)
          (`SplineMeshComponent.SetEndRoll` _returnvalue_6 (/ (`SplineComponent.GetRollAtSplinePoint` _lifeline_spline_6 1 "World") 90.0) true))
        (:`then_1`
          ;[0 1 0.09921] End
          (bind _returnvalue_7 (`AddComponent|NODE_AddSplineMeshComponent-7`))
          (`StaticMeshComponent.SetStaticMesh` _returnvalue_7 (`self.Line Mesh`))
          (`MeshComponent.SetVectorParameterValueOnMaterials` _returnvalue_7 "Color" (`KismetMathLibrary.Conv_LinearColorToVector` (`self.Color`)))
          (`MeshComponent.SetScalarParameterValueOnMaterials` _returnvalue_7 "Start / End" 1.0)
          (`MeshComponent.SetScalarParameterValueOnMaterials` _returnvalue_7 "Switch" 0.0)
          (`SplineMeshComponent.SetStartAndEnd` _returnvalue_7 _location_4 _tangent_4 _location_3 _tangent_3 true)
          (`SplineMeshComponent.SetEndScale` _returnvalue_7 _returnvalue true)
          (`SplineMeshComponent.SetStartScale` _returnvalue_7 _scale_2 true)
          (`SplineMeshComponent.SetStartRoll` _returnvalue_7 (/ (`SplineComponent.GetRollAtSplinePoint` _lifeline_spline_5 _returnvalue_3 "World") 90.0) true)
          (`SplineMeshComponent.SetEndRoll` _returnvalue_7 (/ (`SplineComponent.GetRollAtSplinePoint` _lifeline_spline_5 _returnvalue_2 "World") 90.0) true))))
    (:`then_1`
      (`ParticleSystemComponent.SetColorParameter` (`self.Line Particle`) "LineColor" (* (`self.Color`) 100.0)))))

(event `Hit Spline`
  (set `self.Active Spline` true)
  (bind _asbp_jin (cast `/Game/Prototype/Blueprints/BP_Jin` (`GameplayStatics.GetPlayerCharacter` 0)))
  (set `/Game/Prototype/Blueprints/BP_Jin.LineSpeed` (`self.Lifeline Speed`) _asbp_jin))

(event `self.ReceiveTick`
  (params (DeltaSeconds :type "Float (single-precision)"))
  (bind (_on_spline_air _on_spline_surface) (`/Game/Prototype/Blueprints/LijarFunctionLibrary.On Spline Mode?`))
  (bind _max_lifeline_energy (`self.Max Lifeline Energy`))
  (if (`self.Active Spline`)
    (bind _asbp_jin (cast `/Game/Prototype/Blueprints/BP_Jin` (`GameplayStatics.GetPlayerCharacter` 0)))
    (if _on_spline_air
      ;[0.1736 0.4896 0.0294] Karma System
      (if _on_spline_surface
        (`KismetSystemLibrary.Delay` (`self.Gain Speed`))
        (bind _aslijar_game_instance (cast `/Game/Prototype/Blueprints/Lijar_Gameinstance` (`GameplayStatics.GetGameInstance`)))
        (bind _returnvalue (/ (`KismetMathLibrary.FClamp` (`KismetMathLibrary.VSize` (`self.GetVelocity` _asbp_jin)) 0.0 4000.0) 4000.0))
        (set `self.Gain Speed` (`KismetMathLibrary.Lerp` 0.1 0.05 _returnvalue))
        (set `self.Lifeline Energy` (`KismetMathLibrary.FClamp` (- (`self.Lifeline Energy`) 1.0) 0.0 (`self.Max Lifeline Energy`)))
        (bind _returnvalue_2 (`KismetMathLibrary.Lerp` 1.0 10.0 _returnvalue))
        (`/Game/Prototype/Blueprints/Lijar_Gameinstance.Karma Update` _aslijar_game_instance (* (`KismetMathLibrary.Lerp` 0.0 (`self.Lifeline Karma Gain`) (/ (`KismetMathLibrary.FClamp` (`self.Lifeline Energy`) 0.0 _max_lifeline_energy) _max_lifeline_energy)) _returnvalue_2) (0.0 0.0 0.0))
        (`/Game/Prototype/Blueprints/BP_Jin.Add Energy` _asbp_jin (* (`self.Lifeline Karma Gain`) _returnvalue_2)))
      (else
        (`KismetSystemLibrary.Delay` 3.0)
        (set `self.Active Spline` false)))))

(fn `Attach to Spline`
  (params (`Own Spline` :type "SplineComponent Object Reference") (`Attach Spline` :type "SplineComponent Object Reference"))
  (for _index (range (`self.Attach Point`) (+ (`SplineComponent.GetNumberOfSplinePoints` `Attach Spline`) 1))
    (bind _returnvalue (- _index (`self.Attach Point`)))
    (bind (_location _tangent) (`SplineComponent.GetLocationAndTangentAtSplinePoint` `Attach Spline` _index "World"))
    (`SplineComponent.SetLocationAtSplinePoint` `Own Spline` _returnvalue (+ _location (+ (* (`SplineComponent.GetUpVectorAtSplinePoint` `Attach Spline` _index "World") 10.0) (* (`SplineComponent.GetRightVectorAtSplinePoint` `Attach Spline` _index "World") 1.0) (* (`SceneComponent.GetForwardVector` `Attach Spline`) 1.0))) "World" true)
    (`SplineComponent.SetSplinePointType` `Own Spline` _returnvalue (`SplineComponent.GetSplinePointType` `Attach Spline` _index) true)
    (`SplineComponent.SetTangentAtSplinePoint` `Own Spline` _returnvalue _tangent "World" true)
    (`SplineComponent.UpdateSpline` `Own Spline`))
  (`KismetSystemLibrary.PrintString` "Last Point")
  (return))

(fn `UserConstructionScript`
  (bind _lifeline_spline (`self.Lifeline Spline`))
  (bind _lifeline_spline_2 (`self.Lifeline Spline`))
  (bind _lifeline_spline_3 (`self.Lifeline Spline`))
  (bind _lifeline_spline_4 (`self.Lifeline Spline`))
  (bind _lifeline_spline_5 (`self.Lifeline Spline`))
  (bind _scale (`self.Scale`))
  (bind _lifeline_spline_6 (`self.Lifeline Spline`))
  (bind _scale_2 (`self.Scale`))
  (bind (_location _tangent) (`SplineComponent.GetLocationAndTangentAtSplinePoint` _lifeline_spline_4 0 "Local"))
  (bind (_location_2 _tangent_2) (`SplineComponent.GetLocationAndTangentAtSplinePoint` _lifeline_spline_4 1 "Local"))
  (bind _returnvalue (* _scale_2 (`self.Start End Pinch`)))
  (bind _returnvalue_2 (`SplineComponent.GetNumberOfSplinePoints` _lifeline_spline_2))
  (bind _spline_mid (`/Game/Prototype/Blueprints/Line/SplineProcedural_BP.Spline Mid` (`self.Oriantation Spline`)))
  (bind _returnvalue_3 (- _returnvalue_2 2))
  (bind (_location_3 _tangent_3) (`SplineComponent.GetLocationAndTangentAtSplinePoint` _lifeline_spline_2 _returnvalue_2 "Local"))
  (bind (_location_4 _tangent_4) (`SplineComponent.GetLocationAndTangentAtSplinePoint` _lifeline_spline_2 _returnvalue_3 "Local"))
  (`|ExecutionSequence`
    (:`then_0`
      (for _index (range (`SplineComponent.GetNumberOfSplinePoints` _spline_mid))
        (bind _returnvalue_4 (`SplineComponent.GetLocationAtSplinePoint` _spline_mid _index "World"))
        (if (== _returnvalue_4 (`self.K2_GetActorLocation`) :`ErrorTolerance` (`self.Snap Tolerance`))
          (bind _output_get (set `self.Attach Location` _returnvalue_4))
          (set `self.Attach Point` _index)
          (set `self.Has Attach Point?` true)
          (if (`self.Has Attach Point?`)
            (`self.K2_SetActorLocation` _output_get)
            (`KismetSystemLibrary.PrintString` "No Attachpoint" true true (struct :`G` 0.66 :`B` 1.0 :`A` 1.0) 0.1)
            (`self.Attach to Spline` (`self.Lifeline Spline`) _spline_mid))
          (else
            (set `self.Has Attach Point?` false)))))
    (:`then_1`
      (`SplineComponent.UpdateSpline` (`self.Lifeline Spline`))
      (`|ExecutionSequence`
        (:`then_0`
          (for _index_2 (range 1 (+ (- (`SplineComponent.GetNumberOfSplinePoints` _lifeline_spline) 3) 1))
            (bind _returnvalue_5 (`AddComponent|NODE_AddSplineMeshComponent-0`))
            (`StaticMeshComponent.SetStaticMesh` _returnvalue_5 (`self.Line Mesh`))
            (`MeshComponent.SetVectorParameterValueOnMaterials` _returnvalue_5 "Color" (`KismetMathLibrary.Conv_LinearColorToVector` (`self.Color`)))
            (bind (_location_5 _tangent_5) (`SplineComponent.GetLocationAndTangentAtSplinePoint` _lifeline_spline _index_2 "Local"))
            (bind _returnvalue_6 (+ _index_2 1))
            (bind (_location_6 _tangent_6) (`SplineComponent.GetLocationAndTangentAtSplinePoint` _lifeline_spline _returnvalue_6 "Local"))
            (`SplineMeshComponent.SetStartAndEnd` _returnvalue_5 _location_5 _tangent_5 _location_6 _tangent_6 true)
            (`SplineMeshComponent.SetStartScale` _returnvalue_5 _scale true)
            (`SplineMeshComponent.SetEndScale` _returnvalue_5 _scale true)
            (`SplineMeshComponent.SetStartRoll` _returnvalue_5 (/ (`SplineComponent.GetRollAtSplinePoint` _lifeline_spline_3 _index_2 "World") 90.0) true)
            (`SplineMeshComponent.SetEndRoll` _returnvalue_5 (/ (`SplineComponent.GetRollAtSplinePoint` _lifeline_spline_3 _returnvalue_6 "World") 90.0) true))
          (`|ExecutionSequence`
            (:`then_0`
              ;[0 0.9671 1] Start
              (bind _returnvalue_7 (`AddComponent|NODE_AddSplineMeshComponent-3`))
              (`StaticMeshComponent.SetStaticMesh` _returnvalue_7 (`self.Line Mesh`))
              (`MeshComponent.SetVectorParameterValueOnMaterials` _returnvalue_7 "Color" (`KismetMathLibrary.Conv_LinearColorToVector` (`self.Color`)))
              (`MeshComponent.SetScalarParameterValueOnMaterials` _returnvalue_7 "Start / End" 0.0)
              (`MeshComponent.SetScalarParameterValueOnMaterials` _returnvalue_7 "Switch" 0.0)
              (`SplineMeshComponent.SetStartAndEnd` _returnvalue_7 _location _tangent _location_2 _tangent_2 true)
              (`SplineMeshComponent.SetStartScale` _returnvalue_7 _returnvalue true)
              (`SplineMeshComponent.SetEndScale` _returnvalue_7 _scale_2 true)
              (`SplineMeshComponent.SetStartRoll` _returnvalue_7 (/ (`SplineComponent.GetRollAtSplinePoint` _lifeline_spline_6 0 "World") 90.0) true)
              (`SplineMeshComponent.SetEndRoll` _returnvalue_7 (/ (`SplineComponent.GetRollAtSplinePoint` _lifeline_spline_6 1 "World") 90.0) true))
            (:`then_1`
              ;[0 1 0.09921] End
              (bind _returnvalue_8 (`AddComponent|NODE_AddSplineMeshComponent-4`))
              (`StaticMeshComponent.SetStaticMesh` _returnvalue_8 (`self.Line Mesh`))
              (`MeshComponent.SetVectorParameterValueOnMaterials` _returnvalue_8 "Color" (`KismetMathLibrary.Conv_LinearColorToVector` (`self.Color`)))
              (`MeshComponent.SetScalarParameterValueOnMaterials` _returnvalue_8 "Start / End" 1.0)
              (`MeshComponent.SetScalarParameterValueOnMaterials` _returnvalue_8 "Switch" 0.0)
              (`SplineMeshComponent.SetStartAndEnd` _returnvalue_8 _location_4 _tangent_4 _location_3 _tangent_3 true)
              (`SplineMeshComponent.SetEndScale` _returnvalue_8 _returnvalue true)
              (`SplineMeshComponent.SetStartScale` _returnvalue_8 _scale_2 true)
              (`SplineMeshComponent.SetStartRoll` _returnvalue_8 (/ (`SplineComponent.GetRollAtSplinePoint` _lifeline_spline_5 _returnvalue_3 "World") 90.0) true)
              (`SplineMeshComponent.SetEndRoll` _returnvalue_8 (/ (`SplineComponent.GetRollAtSplinePoint` _lifeline_spline_5 _returnvalue_2 "World") 90.0) true))))
        (:`then_1`
          (`ParticleSystemComponent.SetColorParameter` (`self.Line Particle`) "LineColor" (* (`self.Color`) 0.0)))))))