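; Lifeline rail actor: a coloured spline line for BP_Jin, with a spawned SnapPoint that tracks the player's position along it at an offset.
; Construction uses the Twist Correct plugin to build offset and corrected splines, lay spline meshes and add debug arrows.
; Tick's speed-scaled karma and energy reward, which drains line energy, sits behind contradictory IsFalling checks.
; Older spline-attach, mesh-building and ground-trace construction code is disconnected.
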(event `Respawn Snap Point`
  (`KismetSystemLibrary.Delay` 3.0)
  (bind _returnvalue (`|SpawnActorFromClass` "/Game/Prototype/Blueprints/Line/SnapPoint_Bp.SnapPoint_Bp_C" (`self.GetTransform`) "Undefined" "OverrideRootScale" null null :!label _label))
  (set `self.Snap Point` _returnvalue))

(event `self.ReceiveBeginPlay`
  (set `self.Lifeline Energy` (`self.Max Lifeline Energy`))
  (goto _label))

(event `Spline Toggle Active`
  (`/Engine/EditorBlueprintResources/StandardMacros.FlipFlop`
    (:`A`
      (set `self.Active Spline` true))
    (:`B`
      (set `self.Active Spline` false))))

(event `self.ReceiveTick`
  (params (DeltaSeconds :type "Float (single-precision)"))
  (bind _returnvalue (`GameplayStatics.GetPlayerCharacter` 0))
  (bind _max_lifeline_energy (`self.Max Lifeline Energy`))
  (bind _spline (`self.Spline`))
  (bind _returnvalue_2 (+ (`/Game/Prototype/Blueprints/LijarFunctionLibrary.Get Actor Distance Along Spline` (`self.Spline`) (`self.K2_GetActorLocation` _returnvalue)) (`self.Snap Point Offset`)))
  (`|ExecutionSequence`
    (:`then_0`
      (if (`self.Active Spline`)
        (bind _asbp_jin (cast `/Game/Prototype/Blueprints/BP_Jin` (`GameplayStatics.GetPlayerCharacter` 0)))
        (bind _isonspline_ (`/Game/Prototype/Blueprints/BP_Jin.IsOnSpline?` _asbp_jin))
        (bind _returnvalue_3 (`NavMovementComponent.IsFalling` (`Character.CharacterMovement` _asbp_jin)))
        (if (and _isonspline_ _returnvalue_3)
          ;[0.1736 0.4896 0.0294] Karma System
          (if (and _isonspline_ (not _returnvalue_3))
            (`KismetSystemLibrary.Delay` (`self.Gain Speed`))
            (bind _aslijar_game_instance (cast `/Game/Prototype/Blueprints/Lijar_Gameinstance` (`GameplayStatics.GetGameInstance`)))
            (bind _returnvalue_4 (/ (`KismetMathLibrary.FClamp` (`KismetMathLibrary.VSize` (`self.GetVelocity` _asbp_jin)) 0.0 4000.0) 4000.0))
            (set `self.Gain Speed` (`KismetMathLibrary.Lerp` 0.1 0.05 _returnvalue_4))
            (set `self.Lifeline Energy` (`KismetMathLibrary.FClamp` (- (`self.Lifeline Energy`) 1.0) 0.0 (`self.Max Lifeline Energy`)))
            (bind _returnvalue_5 (`KismetMathLibrary.Lerp` 1.0 10.0 _returnvalue_4))
            (`/Game/Prototype/Blueprints/Lijar_Gameinstance.Karma Update` _aslijar_game_instance (* (`KismetMathLibrary.Lerp` 0.0 (`self.Lifeline Karma Gain`) (/ (`KismetMathLibrary.FClamp` (`self.Lifeline Energy`) 0.0 _max_lifeline_energy) _max_lifeline_energy)) _returnvalue_5) (0.0 0.0 0.0))
            (`/Game/Prototype/Blueprints/BP_Jin.Add Energy` _asbp_jin (* (`self.Lifeline Karma Gain`) _returnvalue_5)))
          (else
            (`KismetSystemLibrary.Delay` 3.0)
            (set `self.Active Spline` false)))))
    (:`then_1`
      (`/Engine/EditorBlueprintResources/StandardMacros.IsValid` _returnvalue
        (:`Is Valid`
          (`SceneComponent.K2_SetWorldLocationAndRotation` (`Actor.RootComponent` (`self.Snap Point`)) (+ (`SplineComponent.GetLocationAtDistanceAlongSpline` _spline _returnvalue_2 "World") (0.0 0.0 100.0)) (`SplineComponent.GetRotationAtDistanceAlongSpline` _spline _returnvalue_2 "World") false false))))))

(fn `Attach Spline`
  (params (`Own Spline` :type "SplineComponent Object Reference") (`Other Spline` :type "SplineComponent Object Reference"))
  (for _index (range (`self.Attach Point`) (+ (`SplineComponent.GetNumberOfSplinePoints` `Other Spline`) 1))
    (bind _returnvalue (- _index (`self.Attach Point`)))
    (bind (_location _tangent) (`SplineComponent.GetLocationAndTangentAtSplinePoint` `Other Spline` _index "World"))
    (`SplineComponent.SetLocationAtSplinePoint` `Own Spline` _returnvalue (+ _location (+ (* (`SplineComponent.GetUpVectorAtSplinePoint` `Other Spline` _index "World") (`self.Z Offset`)) (* (`SplineComponent.GetRightVectorAtSplinePoint` `Other Spline` _index "World") 1.0) (* (`SceneComponent.GetForwardVector` `Other Spline`) 1.0))) "World" true)
    (`SplineComponent.SetSplinePointType` `Own Spline` _returnvalue (`SplineComponent.GetSplinePointType` `Other Spline` _index) true)
    (`SplineComponent.SetTangentAtSplinePoint` `Own Spline` _returnvalue _tangent "World" true)))

(fn `Debug Spline Vector`
  (params (Spline :type "SplineComponent Object Reference"))
  (for _index (range (`SplineComponent.GetNumberOfSplinePoints` Spline))
    (`SplineComponent.SetUpVectorAtSplinePoint` Spline _index (`SplineComponent.GetUpVectorAtSplinePoint` Spline _index "Local") "Local" true)
    (bind _returnvalue (`SplineComponent.GetLocationAtSplinePoint` Spline _index "Local"))
    (bind _returnvalue_2 (`SplineComponent.GetUpVectorAtSplinePoint` Spline _index "Local"))
    (bind _returnvalue_3 (`AddComponent|NODE_AddArrowComponent-1` :`RelativeTransform` (`KismetMathLibrary.MakeTransform` _returnvalue (`KismetMathLibrary.Conv_VectorToRotator` _returnvalue_2))))
    (`ArrowComponent.SetArrowColor` _returnvalue_3 (struct :`B` 1.0 :`A` 1.0))
    (bind _returnvalue_4 (`SplineComponent.GetRightVectorAtSplinePoint` Spline _index "Local"))
    (bind _returnvalue_5 (`AddComponent|NODE_AddArrowComponent-2` :`RelativeTransform` (`KismetMathLibrary.MakeTransform` _returnvalue (`KismetMathLibrary.Conv_VectorToRotator` _returnvalue_4))))
    (`ArrowComponent.SetArrowColor` _returnvalue_5 (struct :`G` 1.0 :`A` 1.0))
    (bind _returnvalue_6 (`AddComponent|NODE_AddArrowComponent-3` :`RelativeTransform` (`KismetMathLibrary.MakeTransform` _returnvalue (`KismetMathLibrary.Conv_VectorToRotator` (* (`KismetMathLibrary.Cross_VectorVector` _returnvalue_2 _returnvalue_4) -1)))))
    (`ArrowComponent.SetArrowColor` _returnvalue_6 (struct :`R` 1.0 :`A` 1.0))))

(fn `Display Arrows`
  (params (`Direction Arrows` :type Boolean) (`Initilize?` :type Boolean) (`Spline to Use` :type "SplineComponent Object Reference"))
  (if `Direction Arrows`
    (if `Initilize?`
      (for _index (range (`SplineComponent.GetNumberOfSplinePoints` `Spline to Use`))
        (bind _returnvalue (`SplineComponent.GetLocationAtSplinePoint` `Spline to Use` _index "Local"))
        (bind _returnvalue_2 (`SplineComponent.GetUpVectorAtSplinePoint` `Spline to Use` _index "Local"))
        (bind _returnvalue_3 (`AddComponent|NODE_AddArrowComponent-4` :`RelativeTransform` (`KismetMathLibrary.MakeTransform` _returnvalue (`KismetMathLibrary.MakeRotFromX` _returnvalue_2))))
        (`KismetArrayLibrary.Array_Set` (`self.Arrows`) _index _returnvalue_3 true)
        (if (`self.Numbers?`)
          (bind _returnvalue_4 (`AddComponent|NODE_AddTextRenderComponent-0` :`RelativeTransform` (`KismetMathLibrary.MakeTransform` (+ (* _returnvalue_2 -30.0) _returnvalue))))
          (`TextRenderComponent.K2_SetText` _returnvalue_4 (`KismetTextLibrary.Conv_IntToText` _index))))
      (else
        (for (_array_element _array_index) (`self.Arrows`)
          (`SceneComponent.K2_SetRelativeRotation` _array_element (`KismetMathLibrary.MakeRotFromX` (- (`SplineComponent.GetLocationAtSplinePoint` (`self.SplineOffset`) _array_index "Local") (`SplineComponent.GetLocationAtSplinePoint` (`self.Spline`) _array_index "Local"))) false false))))))

(fn `Twist Correct`
  (bind _number (`self.Number`))
  (bind _splinemesh (`self.SplineMesh`))
  (bind (_number_2 _length) (`self.CalcRailLength` (`self.SplineFinal`) (`self.IdealLength`)))
  (bind _output (`|GetArrayItem` _splinemesh))
  (bind _output_2 (`|GetArrayItem` _splinemesh (- (`KismetArrayLibrary.Array_Length` _splinemesh) 1)))
  (`|ExecutionSequence`
    (:`then_0`
      (bind _returnvalue (`AddComponent|NODE_AddSplineComponent-0`))
      (bind _output_get (set `self.SplineOffset` _returnvalue))
      (`SplineComponent.SetClosedLoop` _output_get (`self.ClosedLoop?`) true)
      ;[1 0.4392 0] Twist Correct Plugin
      (`self.BuildOffsetSpline` (`self.Spline`) (`self.SplineOffset`) 0.0 40.0))
    (:`then_1`
      (bind _returnvalue_2 (`AddComponent|NODE_AddSplineComponent-1`))
      (bind _output_get_2 (set `self.SplineFinal` _returnvalue_2))
      (`SplineComponent.SetClosedLoop` _output_get_2 (`self.ClosedLoop?`) true)
      (`self.BuildCorrectedSpline` (`self.Spline`) (`self.SplineOffset`) (`self.SplineFinal`) (`self.IdealLength`)))
    (:`then_2`
      (set `self.Number` _number_2)
      (set `self.Length` _length)
      (`KismetArrayLibrary.Array_Resize` (`self.SplineMesh`) _number)
      (for _index (range _number)
        (set `self.Index` _index)
        (bind _returnvalue_3 (`AddComponent|NODE_AddSplineMeshComponent-5`))
        ;[1 0.4392 0] Twist Correct Plugin
        (`self.ConfigSplineMesh` (`self.Index`) (`self.Length`) (`self.SplineFinal`) _returnvalue_3 self "/Game/Prototype/Particles/Materials/M_Line_Inst.M_Line_Inst" "/Game/Prototype/Meshes/Line.Line")
        ;[1 1 1] Used only for event graph
        (`KismetArrayLibrary.Array_Set` (`self.SplineMesh`) (`self.Index`) _returnvalue_3)
        (`MeshComponent.SetVectorParameterValueOnMaterials` _returnvalue_3 "Color" (`KismetMathLibrary.Conv_LinearColorToVector` (`self.Color`))))
      ;[0 0.771 1] Start End Parameters
      (`MeshComponent.SetScalarParameterValueOnMaterials` _output "Start / End" 0.0)
      (`MeshComponent.SetScalarParameterValueOnMaterials` _output "Switch" 0.0)
      (`MeshComponent.SetScalarParameterValueOnMaterials` _output_2 "Start / End" 1.0)
      (`MeshComponent.SetScalarParameterValueOnMaterials` _output_2 "Switch" 0.0))))

(fn `UserConstructionScript`
  (set `self.ClosedLoop?` (`SplineComponent.IsClosedLoop` (`self.Spline`)))
  (`self.Twist Correct`)
  (`self.Display Arrows` true true (`self.Spline`)))