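; Prototype debug actor for inspecting spline orientation and spline mesh generation.
; The construction script tiles spline meshes at fixed spacing, shrinking tangents on the last partial segment, then draws colored up, right and forward arrows along the spline.
; At BeginPlay a timeline moves a cube along the spline, rotated to an up/right/forward frame built from spline vectors.
; Roll and up-direction correction logic is present but disconnected.
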(event `self.ReceiveBeginPlay`
  (bind _spline (`self.Spline`))
  (bind (_direction _move) (`Timeline|Timeline Move`)
    (:`Update`
      (bind _output_get (set `self.Distance` (* _move (`SplineComponent.GetSplineLength` _spline))))
      (bind _returnvalue (`SplineComponent.GetUpVectorAtDistanceAlongSpline` _spline _output_get "Local"))
      (bind _returnvalue_2 (`SplineComponent.GetRightVectorAtDistanceAlongSpline` _spline _output_get "Local"))
      (`SceneComponent.K2_SetRelativeLocationAndRotation` (`self.Cube`) (`SplineComponent.GetLocationAtDistanceAlongSpline` _spline _output_get "Local") (`KismetMathLibrary.MakeRotationFromAxes` (* (`KismetMathLibrary.Cross_VectorVector` _returnvalue _returnvalue_2) -1) _returnvalue_2 _returnvalue) false false))
    (:`Finished`
      (`KismetSystemLibrary.PrintString` "Done"))))

(fn `UserConstructionScript`
  (bind _mesh_component (`self.Mesh Component`))
  (bind _coordinate_space (`self.Coordinate Space`))
  (bind (_remainder _returnvalue) (`KismetMathLibrary.FMod` (`SplineComponent.GetSplineLength` (`self.Spline`)) (`self.Spacing`)))
  (for _index (range (+ _returnvalue 1))
    (bind _output_get (set `self.Segment Index` _index))
    (set `self.Final Tangent Scale` (select `bool` (== _output_get _returnvalue) :`false` (`self.Tangent Scale`) :`true` (* (/ _remainder (`self.Spacing`)) (`self.Tangent Scale`))))
    (bind _output_get_2 (set `self.Start Distance` (* (`self.Segment Index`) (`self.Spacing`))))
    (set `self.Middle Distance` (+ _output_get_2 (* (`self.Spacing`) 0.5)))
    (set `self.End Distance` (+ (`self.Start Distance`) (`self.Spacing`)))
    (bind _returnvalue_2 (`AddComponent|NODE_AddSplineMeshComponent-1`))
    (bind _output_get_3 (set `self.Mesh Component` _returnvalue_2))
    (`StaticMeshComponent.SetStaticMesh` _output_get_3 (`self.Mesh`))
    (`PrimitiveComponent.SetMaterial` _output_get_3 0 (`self.Material`))
    (`SplineMeshComponent.SetStartAndEnd` (`self.Mesh Component`) (`SplineComponent.GetLocationAtDistanceAlongSpline` (`self.Spline`) (`self.Start Distance`) _coordinate_space) (* (`SplineComponent.GetDirectionAtDistanceAlongSpline` (`self.Spline`) (`self.Start Distance`) _coordinate_space) (`self.Final Tangent Scale`)) (`SplineComponent.GetLocationAtDistanceAlongSpline` (`self.Spline`) (`self.End Distance`) _coordinate_space) (* (`SplineComponent.GetDirectionAtDistanceAlongSpline` (`self.Spline`) (`self.End Distance`) _coordinate_space) (`self.Final Tangent Scale`)) true)
    (`SplineMeshComponent.SetStartScale` _mesh_component (`KismetMathLibrary.MakeVector2D` (.y (`SplineComponent.GetScaleAtDistanceAlongSpline` (`self.Spline`) (`self.Start Distance`))) (.z (`SplineComponent.GetScaleAtDistanceAlongSpline` (`self.Spline`) (`self.Start Distance`)))) true)
    (`SplineMeshComponent.SetEndScale` _mesh_component (`KismetMathLibrary.MakeVector2D` (.y (`SplineComponent.GetScaleAtDistanceAlongSpline` (`self.Spline`) (`self.End Distance`))) (.z (`SplineComponent.GetScaleAtDistanceAlongSpline` (`self.Spline`) (`self.End Distance`)))) true))
  (`self.Visualize Spline  Vectors` (`self.Spline`) (`self.Steps`)))

(fn `Visualize Spline  Vectors`
  (params (Target :type "SplineComponent Object Reference") (Steps :type Integer :default 25))
  (for _index (range (+ (/ (`KismetMathLibrary.FTrunc` (`SplineComponent.GetSplineLength` Target)) Steps) 1))
    (bind _output_get (set `self.Distance` (`KismetMathLibrary.Conv_IntToDouble` (* _index Steps))))
    (bind _returnvalue (`SplineComponent.GetLocationAtDistanceAlongSpline` Target _output_get "Local"))
    (bind _returnvalue_2 (`SplineComponent.GetUpVectorAtDistanceAlongSpline` Target _output_get "Local"))
    (bind _returnvalue_3 (`AddComponent|NODE_AddArrowComponent-0` :`RelativeTransform` (`KismetMathLibrary.MakeTransform` _returnvalue (`KismetMathLibrary.Conv_VectorToRotator` _returnvalue_2))))
    (`ArrowComponent.SetArrowColor` _returnvalue_3 (struct :`B` 1.0 :`A` 1.0))
    (bind _returnvalue_4 (`SplineComponent.GetRightVectorAtDistanceAlongSpline` Target _output_get "Local"))
    (bind _returnvalue_5 (`AddComponent|NODE_AddArrowComponent-3` :`RelativeTransform` (`KismetMathLibrary.MakeTransform` _returnvalue (`KismetMathLibrary.Conv_VectorToRotator` _returnvalue_4))))
    (`ArrowComponent.SetArrowColor` _returnvalue_5 (struct :`G` 1.0 :`A` 1.0))
    (bind _returnvalue_6 (`AddComponent|NODE_AddArrowComponent-4` :`RelativeTransform` (`KismetMathLibrary.MakeTransform` _returnvalue (`KismetMathLibrary.Conv_VectorToRotator` (* (`KismetMathLibrary.Cross_VectorVector` _returnvalue_2 _returnvalue_4) -1)))))
    (`ArrowComponent.SetArrowColor` _returnvalue_6 (struct :`R` 1.0 :`A` 1.0))))