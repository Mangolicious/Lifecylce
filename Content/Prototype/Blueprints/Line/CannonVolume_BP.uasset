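; CannonVolume_BP is a launch volume that fires the BP_Jin character along an arrow's direction.
; When BP_Jin overlaps the Sphere, it adds an impulse to the character movement along the Arrow's forward vector, scaled by LaunchSpeed, with a VelocityChange toggle.
; It also spawns a bounce particle at the volume, pitched relative to that direction, and attaches a trail particle to the character's mesh.
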(event `self.Sphere.OnComponentBeginOverlap`
  (params (OverlappedComponent :type "PrimitiveComponent Object Reference") (OtherActor :type "Actor Object Reference") (OtherComp :type "PrimitiveComponent Object Reference") (OtherBodyIndex :type Integer) (bFromSweep :type Boolean) (SweepResult :type "HitResult Structure (by ref)"))
  (bind _returnvalue (`KismetMathLibrary.Normal` (`SceneComponent.GetForwardVector` (`self.Arrow`))))
  (bind _returnvalue_2 (`KismetMathLibrary.Conv_VectorToRotator` _returnvalue))
  (`/Engine/EditorBlueprintResources/StandardMacros.IsValid` OtherActor
    (:`Is Valid`
      (bind _asbp_jin (cast `/Game/Prototype/Blueprints/PlayerCharacter/BP_Jin` OtherActor))
      (`CharacterMovementComponent.AddImpulse` (`Character.CharacterMovement` _asbp_jin) (* _returnvalue (`self.Launch Speed`)) (`self.Velocity Change`))
      (`GameplayStatics.SpawnEmitterAtLocation` "/Game/Prototype/Particles/P_Bounce.P_Bounce" (`self.K2_GetActorLocation`) (`KismetMathLibrary.MakeRotator` (.roll _returnvalue_2) (+ (.pitch _returnvalue_2) -90.0) (.yaw _returnvalue_2)))
      (`GameplayStatics.SpawnEmitterAttached` "/Game/Prototype/Particles/P_CharacterTrails.P_CharacterTrails" (`Character.Mesh` _asbp_jin) "None" (0.0 0.0 0.0) (`KismetMathLibrary.MakeRotator` 0.0 0.0 (.yaw _returnvalue_2))))))

(fn `UserConstructionScript`)