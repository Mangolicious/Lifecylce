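; Prototype spline actor that builds a colored lifeline road at construction.
; One spline mesh per segment forms the road, overlaid by a line with separate start, middle and end meshes, the caps pinched by StartEndPinch.
; All pieces follow the spline's tangents, scale and roll, and take the Color material parameter.
; Line pieces are stored in MeshArray for roll animation, but that event-graph logic is unconnected and never runs.
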(fn `UserConstructionScript`
  (bind _spline (`self.Spline`))
  (bind _spline_2 (`self.Spline`))
  (bind _spline_3 (`self.Spline`))
  (bind _spline_4 (`self.Spline`))
  (bind _scale (`self.Scale`))
  (bind _start_end_pinch (`self.Start End Pinch`))
  (bind _scale_2 (`self.Scale`))
  (bind _spline_5 (`self.Spline`))
  (bind _spline_6 (`self.Spline`))
  (bind _spline_7 (`self.Spline`))
  (bind _scale_3 (`self.Scale`))
  (bind _spline_8 (`self.Spline`))
  (bind _scale_4 (`self.Scale`))
  (bind _spline_9 (`self.Spline`))
  (bind _spline_10 (`self.Spline`))
  (bind _start_end_pinch_2 (`self.Start End Pinch`))
  (bind (_returnvalue_x _returnvalue_y) (`KismetMathLibrary.BreakVector` (`SplineComponent.GetScaleAtSplinePoint` _spline_3 0)))
  (bind (_returnvalue_x_2 _returnvalue_y_2) (`KismetMathLibrary.BreakVector` (`SplineComponent.GetScaleAtSplinePoint` _spline_3 1)))
  (bind _returnvalue (`SplineComponent.GetNumberOfSplinePoints` _spline_9))
  (bind (_location _tangent) (`SplineComponent.GetLocationAndTangentAtSplinePoint` _spline_6 0 "Local"))
  (bind (_location_2 _tangent_2) (`SplineComponent.GetLocationAndTangentAtSplinePoint` _spline_6 1 "Local"))
  (bind _returnvalue_2 (`SplineComponent.GetNumberOfSplinePoints` _spline_2))
  (bind _returnvalue_3 (- _returnvalue_2 2))
  (bind (_location_3 _tangent_3) (`SplineComponent.GetLocationAndTangentAtSplinePoint` _spline_2 _returnvalue_2 "Local"))
  (bind (_returnvalue_x_3 _returnvalue_y_3) (`KismetMathLibrary.BreakVector` (`SplineComponent.GetScaleAtSplinePoint` _spline_5 _returnvalue_2)))
  (bind (_location_4 _tangent_4) (`SplineComponent.GetLocationAndTangentAtSplinePoint` _spline_2 _returnvalue_3 "Local"))
  (bind (_returnvalue_x_4 _returnvalue_y_4) (`KismetMathLibrary.BreakVector` (`SplineComponent.GetScaleAtSplinePoint` _spline_5 _returnvalue_3)))
  (`|ExecutionSequence`
    (:`then_0`
      (for _index (range (+ (- _returnvalue 2) 1))
        ;[1 0 0.3522] Road
        (bind _returnvalue_4 (`AddComponent|NODE_AddSplineMeshComponent-5`))
        (`StaticMeshComponent.SetStaticMesh` _returnvalue_4 (`self.Line Mesh`))
        (`MeshComponent.SetVectorParameterValueOnMaterials` _returnvalue_4 "Color" (`KismetMathLibrary.Conv_LinearColorToVector` (`self.Color`)))
        (bind (_location_5 _tangent_5) (`SplineComponent.GetLocationAndTangentAtSplinePoint` _spline _index "Local"))
        (bind _returnvalue_5 (+ _index 1))
        (bind (_location_6 _tangent_6) (`SplineComponent.GetLocationAndTangentAtSplinePoint` _spline _returnvalue_5 "Local"))
        (`SplineMeshComponent.SetStartAndEnd` _returnvalue_4 _location_5 _tangent_5 _location_6 _tangent_6 true)
        (bind (_returnvalue_x_5 _returnvalue_y_5) (`KismetMathLibrary.BreakVector` (`SplineComponent.GetScaleAtSplinePoint` _spline_4 _index)))
        (`SplineMeshComponent.SetStartScale` _returnvalue_4 (* _scale_4 (`KismetMathLibrary.MakeVector2D` _returnvalue_x_5 _returnvalue_y_5)) true)
        (bind (_returnvalue_x_6 _returnvalue_y_6) (`KismetMathLibrary.BreakVector` (`SplineComponent.GetScaleAtSplinePoint` _spline_4 _returnvalue_5)))
        (`SplineMeshComponent.SetEndScale` _returnvalue_4 (* _scale_4 (`KismetMathLibrary.MakeVector2D` _returnvalue_x_6 _returnvalue_y_6)) true)
        (`SplineMeshComponent.SetStartRoll` _returnvalue_4 (/ (`SplineComponent.GetRollAtSplinePoint` _spline_4 _index "World") 90.0) true)
        (`SplineMeshComponent.SetEndRoll` _returnvalue_4 (/ (`SplineComponent.GetRollAtSplinePoint` _spline_4 _returnvalue_5 "World") 90.0) true)))
    (:`then_1`
      (for _index_2 (range 1 (+ (- _returnvalue 3) 1))
        ;[0 0.1458 1] Middle
        (bind _returnvalue_6 (`AddComponent|NODE_AddSplineMeshComponent-0`))
        (`KismetArrayLibrary.Array_Add` (`self.Mesh Array`) _returnvalue_6)
        (`StaticMeshComponent.SetStaticMesh` _returnvalue_6 (`self.Line Mesh Middle`))
        (`MeshComponent.SetVectorParameterValueOnMaterials` _returnvalue_6 "Color" (`KismetMathLibrary.Conv_LinearColorToVector` (`self.Color`)))
        (bind (_location_7 _tangent_7) (`SplineComponent.GetLocationAndTangentAtSplinePoint` _spline_9 _index_2 "Local"))
        (bind _returnvalue_7 (+ _index_2 1))
        (bind (_location_8 _tangent_8) (`SplineComponent.GetLocationAndTangentAtSplinePoint` _spline_9 _returnvalue_7 "Local"))
        (`SplineMeshComponent.SetStartAndEnd` _returnvalue_6 _location_7 _tangent_7 _location_8 _tangent_8 true)
        (bind (_returnvalue_x_7 _returnvalue_y_7) (`KismetMathLibrary.BreakVector` (`SplineComponent.GetScaleAtSplinePoint` _spline_8 _index_2)))
        (`SplineMeshComponent.SetStartScale` _returnvalue_6 (* _scale_3 (`KismetMathLibrary.MakeVector2D` _returnvalue_x_7 _returnvalue_y_7)) true)
        (bind (_returnvalue_x_8 _returnvalue_y_8) (`KismetMathLibrary.BreakVector` (`SplineComponent.GetScaleAtSplinePoint` _spline_8 _returnvalue_7)))
        (`SplineMeshComponent.SetEndScale` _returnvalue_6 (* _scale_3 (`KismetMathLibrary.MakeVector2D` _returnvalue_x_8 _returnvalue_y_8)) true)
        (`SplineMeshComponent.SetStartRoll` _returnvalue_6 (/ (`SplineComponent.GetRollAtSplinePoint` _spline_8 _index_2 "World") 90.0) true)
        (`SplineMeshComponent.SetEndRoll` _returnvalue_6 (/ (`SplineComponent.GetRollAtSplinePoint` _spline_8 _returnvalue_7 "World") 90.0) true))
      (`|ExecutionSequence`
        (:`then_0`
          ;[0 0.9671 1] Start
          (bind _returnvalue_8 (`AddComponent|NODE_AddSplineMeshComponent-3`))
          (`KismetArrayLibrary.Array_Add` (`self.Mesh Array`) _returnvalue_8)
          (`StaticMeshComponent.SetStaticMesh` _returnvalue_8 (`self.Line Mesh Start`))
          (`MeshComponent.SetVectorParameterValueOnMaterials` _returnvalue_8 "Color" (`KismetMathLibrary.Conv_LinearColorToVector` (`self.Color`)))
          (`SplineMeshComponent.SetStartAndEnd` _returnvalue_8 _location _tangent _location_2 _tangent_2 true)
          (`SplineMeshComponent.SetStartScale` _returnvalue_8 (* (* _scale (`KismetMathLibrary.MakeVector2D` _returnvalue_x _returnvalue_y)) _start_end_pinch) true)
          (`SplineMeshComponent.SetEndScale` _returnvalue_8 (* (* _scale (`KismetMathLibrary.MakeVector2D` _returnvalue_x_2 _returnvalue_y_2)) _start_end_pinch) true)
          (`SplineMeshComponent.SetStartRoll` _returnvalue_8 (/ (`SplineComponent.GetRollAtSplinePoint` _spline_10 0 "World") 90.0) true)
          (`SplineMeshComponent.SetEndRoll` _returnvalue_8 (/ (`SplineComponent.GetRollAtSplinePoint` _spline_10 1 "World") 90.0) true))
        (:`then_1`
          ;[0 1 0.09921] End
          (bind _returnvalue_9 (`AddComponent|NODE_AddSplineMeshComponent-4`))
          (`KismetArrayLibrary.Array_Add` (`self.Mesh Array`) _returnvalue_9)
          (`StaticMeshComponent.SetStaticMesh` _returnvalue_9 (`self.Line Mesh End`))
          (`MeshComponent.SetVectorParameterValueOnMaterials` _returnvalue_9 "Color" (`KismetMathLibrary.Conv_LinearColorToVector` (`self.Color`)))
          (`SplineMeshComponent.SetStartAndEnd` _returnvalue_9 _location_4 _tangent_4 _location_3 _tangent_3 true)
          (`SplineMeshComponent.SetEndScale` _returnvalue_9 (* (* _scale_2 (`KismetMathLibrary.MakeVector2D` _returnvalue_x_3 _returnvalue_y_3)) _start_end_pinch_2) true)
          (`SplineMeshComponent.SetStartScale` _returnvalue_9 (* (* _scale_2 (`KismetMathLibrary.MakeVector2D` _returnvalue_x_4 _returnvalue_y_4)) _start_end_pinch_2) true)
          (`SplineMeshComponent.SetStartRoll` _returnvalue_9 (/ (`SplineComponent.GetRollAtSplinePoint` _spline_7 _returnvalue_3 "World") 90.0) true)
          (`SplineMeshComponent.SetEndRoll` _returnvalue_9 (/ (`SplineComponent.GetRollAtSplinePoint` _spline_7 _returnvalue_2 "World") 90.0) true))))))