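; River actor that builds its mesh along an editable spline in the construction script.
; It adds a spline mesh component per segment, using separate start and end meshes for the first and last segments and a repeated mesh between.
; Each segment takes position, tangent, cross-section scale and roll from its spline points.
; An uncalled debug function draws colored arrows for each point's up, right and derived forward axes.
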(fn `Debug Spline Vector`
  (params (Spline :type "SplineComponent Object Reference"))
  (for _index (range (`SplineComponent.GetNumberOfSplinePoints` Spline))
    (`SplineComponent.SetUpVectorAtSplinePoint` Spline _index (`SplineComponent.GetUpVectorAtSplinePoint` Spline _index "Local") "Local" true)
    (bind _returnvalue (`SplineComponent.GetLocationAtSplinePoint` Spline _index "Local"))
    (bind _returnvalue_2 (`SplineComponent.GetUpVectorAtSplinePoint` Spline _index "Local"))
    (bind _returnvalue_3 (`AddComponent|NODE_AddArrowComponent-1` :`RelativeTransform` (`KismetMathLibrary.MakeTransform` _returnvalue (`KismetMathLibrary.Conv_VectorToRotator` _returnvalue_2))))
    (`ArrowComponent.SetArrowColor` _returnvalue_3 (struct :`B` 1.0 :`A` 1.0))
    (bind _returnvalue_4 (`SplineComponent.GetRightVectorAtSplinePoint` Spline _index "Local"))
    (bind _returnvalue_5 (`AddComponent|NODE_AddArrowComponent-2` :`RelativeTransform` (`KismetMathLibrary.MakeTransform` _returnvalue (`KismetMathLibrary.Conv_VectorToRotator` _returnvalue_4))))
    (`ArrowComponent.SetArrowColor` _returnvalue_5 (struct :`G` 1.0 :`A` 1.0))
    (bind _returnvalue_6 (`AddComponent|NODE_AddArrowComponent-3` :`RelativeTransform` (`KismetMathLibrary.MakeTransform` _returnvalue (`KismetMathLibrary.Conv_VectorToRotator` (* (`KismetMathLibrary.Cross_VectorVector` _returnvalue_2 _returnvalue_4) -1)))))
    (`ArrowComponent.SetArrowColor` _returnvalue_6 (struct :`R` 1.0 :`A` 1.0))))

(fn `NewFunction_0`)

(fn `UserConstructionScript`
  (bind _spline (`self.Spline`))
  (bind _spline_2 (`self.Spline`))
  (bind _spline_3 (`self.Spline`))
  (bind _spline_4 (`self.Spline`))
  (bind _spline_5 (`self.Spline`))
  (bind _spline_6 (`self.Spline`))
  (bind (_location _tangent) (`SplineComponent.GetLocationAndTangentAtSplinePoint` _spline_4 1 "Local"))
  (bind (_location_2 _tangent_2) (`SplineComponent.GetLocationAndTangentAtSplinePoint` _spline_4 0 "Local"))
  (bind _returnvalue (`SplineComponent.GetNumberOfSplinePoints` _spline_3))
  (bind _returnvalue_2 (- _returnvalue 2))
  (bind (_location_3 _tangent_3) (`SplineComponent.GetLocationAndTangentAtSplinePoint` _spline_3 _returnvalue "Local"))
  (bind (_location_4 _tangent_4) (`SplineComponent.GetLocationAndTangentAtSplinePoint` _spline_3 _returnvalue_2 "Local"))
  (for _index (range 1 (+ (- (`SplineComponent.GetNumberOfSplinePoints` _spline) 3) 1))
    (bind _returnvalue_3 (`AddComponent|NODE_AddSplineMeshComponent-0`))
    (`StaticMeshComponent.SetStaticMesh` _returnvalue_3 (`self.Mesh`))
    (bind (_location_5 _tangent_5) (`SplineComponent.GetLocationAndTangentAtSplinePoint` _spline _index "Local"))
    (bind _returnvalue_4 (+ _index 1))
    (bind (_location_6 _tangent_6) (`SplineComponent.GetLocationAndTangentAtSplinePoint` _spline _returnvalue_4 "Local"))
    (`SplineMeshComponent.SetStartAndEnd` _returnvalue_3 _location_5 _tangent_5 _location_6 _tangent_6 true)
    (`SplineMeshComponent.SetStartScale` _returnvalue_3 (`KismetMathLibrary.MakeVector2D` (.y (`SplineComponent.GetScaleAtSplinePoint` (`self.Spline`) _index)) (.z (`SplineComponent.GetScaleAtSplinePoint` (`self.Spline`) _index))) true)
    (`SplineMeshComponent.SetEndScale` _returnvalue_3 (`KismetMathLibrary.MakeVector2D` (.y (`SplineComponent.GetScaleAtSplinePoint` (`self.Spline`) _returnvalue_4)) (.z (`SplineComponent.GetScaleAtSplinePoint` (`self.Spline`) _returnvalue_4))) true)
    (`SplineMeshComponent.SetStartRoll` _returnvalue_3 (`KismetMathLibrary.DegreesToRadians` (.roll (`SplineComponent.GetRotationAtSplinePoint` _spline_2 _index "Local"))) true)
    (`SplineMeshComponent.SetEndRoll` _returnvalue_3 (`KismetMathLibrary.DegreesToRadians` (.roll (`SplineComponent.GetRotationAtSplinePoint` _spline_2 (+ _index 1) "Local"))) true))
  (`|ExecutionSequence`
    (:`then_0`
      ;[0 0.9671 1] Start
      (bind _returnvalue_5 (`AddComponent|NODE_AddSplineMeshComponent-3`))
      (`StaticMeshComponent.SetStaticMesh` _returnvalue_5 (`self.Start Mesh`))
      (`SplineMeshComponent.SetStartAndEnd` _returnvalue_5 _location_2 _tangent_2 _location _tangent true)
      (`SplineMeshComponent.SetStartScale` _returnvalue_5 (`KismetMathLibrary.MakeVector2D` (.y (`SplineComponent.GetScaleAtSplinePoint` (`self.Spline`) 0)) (.z (`SplineComponent.GetScaleAtSplinePoint` (`self.Spline`) 0))) true)
      (`SplineMeshComponent.SetEndScale` _returnvalue_5 (`KismetMathLibrary.MakeVector2D` (.y (`SplineComponent.GetScaleAtSplinePoint` (`self.Spline`) 1)) (.z (`SplineComponent.GetScaleAtSplinePoint` (`self.Spline`) 1))) true)
      (`SplineMeshComponent.SetStartRoll` _returnvalue_5 (`KismetMathLibrary.DegreesToRadians` (.roll (`SplineComponent.GetRotationAtSplinePoint` _spline_6 0 "Local"))) true)
      (`SplineMeshComponent.SetEndRoll` _returnvalue_5 (`KismetMathLibrary.DegreesToRadians` (.roll (`SplineComponent.GetRotationAtSplinePoint` _spline_6 1 "Local"))) true))
    (:`then_1`
      ;[0 1 0.09921] End
      (bind _returnvalue_6 (`AddComponent|NODE_AddSplineMeshComponent-4`))
      (`StaticMeshComponent.SetStaticMesh` _returnvalue_6 (`self.End Mesh`))
      (`SplineMeshComponent.SetStartAndEnd` _returnvalue_6 _location_4 _tangent_4 _location_3 _tangent_3 true)
      (`SplineMeshComponent.SetEndScale` _returnvalue_6 (`KismetMathLibrary.MakeVector2D` (.y (`SplineComponent.GetScaleAtSplinePoint` (`self.Spline`) (- _returnvalue 1))) (.z (`SplineComponent.GetScaleAtSplinePoint` (`self.Spline`) (- _returnvalue 1)))) true)
      (`SplineMeshComponent.SetStartScale` _returnvalue_6 (`KismetMathLibrary.MakeVector2D` (.y (`SplineComponent.GetScaleAtSplinePoint` (`self.Spline`) _returnvalue_2)) (.z (`SplineComponent.GetScaleAtSplinePoint` (`self.Spline`) _returnvalue_2))) true)
      (`SplineMeshComponent.SetStartRoll` _returnvalue_6 (`KismetMathLibrary.DegreesToRadians` (.roll (`SplineComponent.GetRotationAtSplinePoint` _spline_5 _returnvalue_2 "Local"))) true)
      (`SplineMeshComponent.SetEndRoll` _returnvalue_6 (`KismetMathLibrary.DegreesToRadians` (.roll (`SplineComponent.GetRotationAtSplinePoint` _spline_5 _returnvalue "Local"))) true))))