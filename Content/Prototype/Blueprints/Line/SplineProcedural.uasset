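; Prototype procedural spline actor that generates a second spline, SplineSide, running alongside its main Spline.
; The construction script rebuilds SplineSide by offsetting each source point along its local right and up vectors, copying point type and tangent.
; BeginPlay is empty; disconnected leftover experiments cover spawning LifeLine_BP, caching point data in arrays and placing debug arrows.
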(event `self.ReceiveBeginPlay`)

(fn `UserConstructionScript`
  (bind _spline_side (`self.Spline Side`))
  (bind _spline (`self.Spline`))
  (`SplineComponent.ClearSplinePoints` (`self.Spline Side`) true)
  (for _index (range (`SplineComponent.GetNumberOfSplinePoints` _spline))
    (bind (_location _tangent) (`SplineComponent.GetLocationAndTangentAtSplinePoint` _spline _index "Local"))
    (`SplineComponent.AddSplinePoint` _spline_side (+ _location (+ (* (`SplineComponent.GetUpVectorAtSplinePoint` _spline _index "Local") 20.0) (* (`SplineComponent.GetRightVectorAtSplinePoint` _spline _index "Local") 100.0) (* (`SceneComponent.GetForwardVector` _spline) 0.0))) "Local" true)
    (`SplineComponent.SetSplinePointType` _spline_side _index (`SplineComponent.GetSplinePointType` _spline _index) true)
    (`SplineComponent.SetTangentAtSplinePoint` _spline_side _index _tangent "Local" true)))