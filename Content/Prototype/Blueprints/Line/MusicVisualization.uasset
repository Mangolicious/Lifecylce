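; Music visualizer actor whose placed instances act as spectrum bars, each with a cube and a randomly colored point light.
; On BeginPlay it gathers all instances and plays the sound on the first one's audio component.
; Each Tick samples the sound's frequency spectrum slightly ahead of game time, mapping cubed band magnitudes by array index to light intensity, hue rotation, cube height and emissive material parameters, recreating dynamic materials every frame.
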(event `self.ReceiveTick`
  (params (DeltaSeconds :type "Float (single-precision)"))
  (bind _outspectrum (`SoundVisualizationStatics.CalculateFrequencySpectrum` (`self.Sound`) 0 (+ (`KismetSystemLibrary.GetGameTimeInSeconds`) 0.08) 0.19 20))
  (bind _output_get (set `self.Frequency` _outspectrum))
  (for (_array_element _array_index) (`self.Actors self`)
    (bind _pointlight (`/Game/Prototype/Blueprints/Line/MusicVisualization.PointLight` _array_element))
    (bind _output (`|GetArrayItem` _output_get _array_index))
    (bind _returnvalue (`KismetMathLibrary.Abs` (* _output _output _output)))
    (bind _returnvalue_2 (+ (* _returnvalue (`self.Intensity`)) 1000.0))
    (`LightComponent.SetIntensity` _pointlight _returnvalue_2)
    (bind _returnvalue_3 (`LightComponentBase.GetLightColor` _pointlight))
    (`LightComponent.SetLightColor` _pointlight (`KismetMathLibrary.Conv_VectorToLinearColor` (`KismetMathLibrary.Normal` (`KismetMathLibrary.RotateAngleAxis` (`KismetMathLibrary.Conv_LinearColorToVector` _returnvalue_3) (* (mod _returnvalue 1.0) 1.0) (1.0 1.0 1.0)))) true)
    (bind _cube (`/Game/Prototype/Blueprints/Line/MusicVisualization.Cube` _array_element))
    (`SceneComponent.SetWorldScale3D` _cube (`KismetMathLibrary.MakeVector` 0.2 0.2 (* (/ _returnvalue_2 50000.0) 5.0)))
    (bind _returnvalue_4 (`PrimitiveComponent.CreateDynamicMaterialInstance` _cube 0 (`PrimitiveComponent.GetMaterial` _cube 0) "None" :!label _label))
    (`MaterialInstanceDynamic.SetScalarParameterValue` _returnvalue_4 "Intensity" (+ (/ _returnvalue_2 1000.0) 10.0))
    (`MaterialInstanceDynamic.SetVectorParameterValue` _returnvalue_4 "Color" _returnvalue_3)))

(event `self.ReceiveBeginPlay`
  (bind _outactors (`GameplayStatics.GetAllActorsOfClass` "MusicVisualization_C"))
  (bind _output_get (set `self.Actors self` _outactors))
  (bind _audio (`/Game/Prototype/Blueprints/Line/MusicVisualization.Audio` (`|GetArrayItem` _output_get)))
  (`AudioComponent.SetSound` _audio (`self.Sound`))
  (`AudioComponent.Play` _audio 0.0)
  (goto _label))

(fn `UserConstructionScript`
  (`LightComponent.SetLightColor` (`self.PointLight`) (`KismetMathLibrary.Conv_VectorToLinearColor` (`KismetMathLibrary.MakeVector` (`KismetMathLibrary.RandomFloatInRange` 0.0 1.0) (`KismetMathLibrary.RandomFloatInRange` 0.0 1.0) (`KismetMathLibrary.RandomFloatInRange` 0.0 1.0))) true))