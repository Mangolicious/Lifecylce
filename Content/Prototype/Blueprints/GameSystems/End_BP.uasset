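; End_BP is a level end trigger that finishes the game when the player character BP_Jin overlaps it.
; On overlap it fades the camera and audio out, holds the fade, then shows the EndScreen widget.
; After a configurable delay it resets CurrentKarma on the Lijar game instance and opens the Menu level.
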(event `self.Trigger.OnComponentBeginOverlap`
  (params (OverlappedComponent :type "PrimitiveComponent Object Reference") (OtherActor :type "Actor Object Reference") (OtherComp :type "PrimitiveComponent Object Reference") (OtherBodyIndex :type Integer) (bFromSweep :type Boolean) (SweepResult :type "HitResult Structure (by ref)"))
  (`/Engine/EditorBlueprintResources/StandardMacros.IsValid` OtherActor
    (:`Is Valid`
      (cast `/Game/Prototype/Blueprints/PlayerCharacter/BP_Jin` OtherActor)
      (`PlayerCameraManager.StartCameraFade` :`self` (`GameplayStatics.GetPlayerCameraManager` (`GameplayStatics.GetPlayerController` 0)) :`ToAlpha` 1.0 :`Duration` 1.0 :`bShouldFadeAudio` true :`bHoldWhenFinished` true)
      (`KismetSystemLibrary.Delay` 1.0)
      (bind _returnvalue (`|CreateWidget` "/Game/Prototype/Blueprints/GameSystems/EndScreen.EndScreen_C" (`GameplayStatics.GetPlayerController` 0)))
      (`UserWidget.AddToViewport` _returnvalue 0)
      (bind _aslijar_game_instance (cast `/Game/Prototype/Blueprints/GameSystems/Lijar_GameInstance` (`GameplayStatics.GetGameInstance`)))
      (`KismetSystemLibrary.Delay` (`self.Delay Till Menu`))
      (set `/Game/Prototype/Blueprints/GameSystems/Lijar_GameInstance.Current Karma` 0.0 _aslijar_game_instance)
      (`GameplayStatics.OpenLevel` "Menu"))))

(fn `UserConstructionScript`)