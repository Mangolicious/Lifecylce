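; Blueprint function library of player-state, spline and actor-search helpers for a game whose player character is BP_Jin.
; Player checks cast player 0 to BP_Jin to report death from Health, or split spline mode into air and surface via IsFalling.
; Spline helpers interpolate distance from the nearest input key and build point rotations from up and right vectors.
; A search scans all actors of a class for the nearest within a distance band.
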(fn `Find Nearest Actor In Range From All Actors Of Class`
  (params (`Actor Class` :type "Actor Class Reference") (Actor :type "Actor Object Reference") (`Minimum Distance` :type "Float (double-precision)") (`Maximum Distance` :type "Float (double-precision)"))
  (returns (`Nearest Actor` :type "Actor Object Reference"))
  (locals (LocalNearestActor :type "Actor Object Reference") (`Closest Distance` :type "Float (double-precision)"))
  (bind _outactors (`GameplayStatics.GetAllActorsOfClass` null `Actor Class`))
  (for _array_element _outactors
    (bind _returnvalue (`Actor.GetDistanceTo` _array_element Actor))
    (if (and (< _returnvalue (`local.Closest Distance`)) (> _returnvalue `Minimum Distance`) (<= _returnvalue `Maximum Distance`))
      (set `local.LocalNearestActor` _array_element)
      (set `local.Closest Distance` _returnvalue)))
  (return (`local.LocalNearestActor`)))

(fn `Get Actor Distance Along Spline`
  (params (`Spline Component` :type "SplineComponent Object Reference") (`Actor World Location` :type "Vector Structure"))
  (returns (`Distance Along Spline` :type "Float (double-precision)"))
  (bind _returnvalue (`SplineComponent.FindInputKeyClosestToWorldLocation` `Spline Component` `Actor World Location`))
  (bind _returnvalue_2 (`KismetMathLibrary.FTrunc` _returnvalue))
  (bind _returnvalue_3 (`SplineComponent.GetDistanceAlongSplineAtSplinePoint` `Spline Component` _returnvalue_2))
  (return (+ _returnvalue_3 (* (- (`SplineComponent.GetDistanceAlongSplineAtSplinePoint` `Spline Component` (`KismetMathLibrary.FTrunc` (+ _returnvalue 1.0))) _returnvalue_3) (- _returnvalue (`KismetMathLibrary.Conv_IntToDouble` _returnvalue_2))))))

(fn `Get Rotation from Axes at Splinepoint`
  (params (Target :type "SplineComponent Object Reference") (PointIndex :type Integer) (CoordinateSpace :type "ESplineCoordinateSpace Enum" :default "Local"))
  (returns (`Return Value` :type "Rotator Structure"))
  (bind _returnvalue (`SplineComponent.GetRightVectorAtSplinePoint` Target PointIndex CoordinateSpace))
  (bind _returnvalue_2 (`SplineComponent.GetUpVectorAtSplinePoint` Target PointIndex CoordinateSpace))
  (return (`KismetMathLibrary.MakeRotationFromAxes` (* (`KismetMathLibrary.Cross_VectorVector` _returnvalue_2 _returnvalue) -1) _returnvalue _returnvalue_2)))

(fn `On Spline Mode?`
  (returns (`On Spline Air` :type Boolean) (`On Spline Surface` :type Boolean))
  (bind _asbp_jin (cast `/Game/Prototype/Blueprints/PlayerCharacter/BP_Jin` (`GameplayStatics.GetPlayerCharacter` null) :!pure true))
  (bind _isonspline_ (`/Game/Prototype/Blueprints/PlayerCharacter/BP_Jin.IsOnSpline?` _asbp_jin))
  (bind _returnvalue (`NavMovementComponent.IsFalling` (`Character.CharacterMovement` _asbp_jin)))
  (return (and _isonspline_ _returnvalue) (and _isonspline_ (not _returnvalue))))

(fn `Player Is Dead?`
  (returns (`Is Dead?` :type Boolean))
  (return (<= (`/Game/Prototype/Blueprints/PlayerCharacter/BP_Jin.Health` (cast `/Game/Prototype/Blueprints/PlayerCharacter/BP_Jin` (`GameplayStatics.GetPlayerCharacter` null) :!pure true)) 0.0)))