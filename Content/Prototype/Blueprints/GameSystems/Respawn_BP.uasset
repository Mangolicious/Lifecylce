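; Respawn_BP is a checkpoint that records itself as the player's respawn point when the player character overlaps its sphere.
; The overlap sets the light intensity via a single FInterpTo step, shows and activates the portal effect, plays a sound, and writes its Index to RespawnIndex in Lijar_GameInstance.
; Its construction script renumbers every Respawn_BP from 1, tags each PlayerStart to match, and labels itself with its Index.
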(event `self.Sphere.OnComponentBeginOverlap`
  (params (OverlappedComponent :type "PrimitiveComponent Object Reference") (OtherActor :type "Actor Object Reference") (OtherComp :type "PrimitiveComponent Object Reference") (OtherBodyIndex :type Integer) (bFromSweep :type Boolean) (SweepResult :type "HitResult Structure (by ref)"))
  (`/Engine/EditorBlueprintResources/StandardMacros.IsValid` OtherActor
    (:`Is Valid`
      (if (== OtherActor (`GameplayStatics.GetPlayerCharacter` 0))
        (`LightComponent.SetIntensity` (`self.PointLight`) (`KismetMathLibrary.FInterpTo` 0.0 (`self.Light Intensity`) (`GameplayStatics.GetWorldDeltaSeconds`) 1.0))
        (`ActorComponent.SetActive` (`self.P_Portal`) true true)
        (`SceneComponent.SetVisibility` (`self.P_Portal`) true false)
        (`GameplayStatics.PlaySoundAtLocation` null (`self.K2_GetActorLocation`) (struct) 1.0 1.0 0.0 null null null)
        (bind _aslijar_game_instance (cast `/Game/Prototype/Blueprints/GameSystems/Lijar_GameInstance` (`GameplayStatics.GetGameInstance`)))
        (bind _output_get (set `/Game/Prototype/Blueprints/GameSystems/Lijar_GameInstance.Respawn Index` (`self.Index`) _aslijar_game_instance))
        (`KismetSystemLibrary.PrintString` (`KismetStringLibrary.Conv_IntToString` _output_get))))))

(fn `UserConstructionScript`
  (bind _returnvalue (`KismetStringLibrary.Conv_IntToString` (`self.Index`)))
  (bind _outactors (`GameplayStatics.GetAllActorsOfClass` "Respawn_BP_C"))
  (for (_array_element _array_index) _outactors
    (bind _output_get (set `/Game/Prototype/Blueprints/GameSystems/Respawn_BP.Index` (+ _array_index 1) _array_element))
    (set `PlayerStart.PlayerStartTag` (`KismetStringLibrary.Conv_StringToName` (`KismetStringLibrary.Conv_IntToString` _output_get)) (`/Game/Prototype/Blueprints/GameSystems/Respawn_BP.Player Start` _array_element)))
  (`KismetSystemLibrary.PrintString` _returnvalue)
  (`TextRenderComponent.K2_SetText` (`self.TextRender`) (`KismetTextLibrary.Conv_StringToText` (`KismetStringLibrary.Concat_StrStr` "Respawn: " _returnvalue))))