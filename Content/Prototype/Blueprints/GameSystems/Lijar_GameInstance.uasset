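; Game instance for the Lijar prototype that holds respawn and karma state.
; SetRespawn stores the respawn index.
; KarmaUpdate adds incoming karma to the current total, scales the whole sum by KarmaMultiplier and clamps it to a non-negative range.
; It also adds the moral delta, scaled by the same multiplier, to an unclamped moral state.
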(event `Set Respawn`
  (params (Index :type Integer))
  (set `self.Respawn Index` Index))

(event `Karma Update`
  (params (Karma :type "Float (double-precision)") (Moral :type "Vector Structure"))
  (bind _karma_multiplier (`self.Karma Multiplier`))
  (set `self.Current Karma` (`KismetMathLibrary.FClamp` (* (+ Karma (`self.Current Karma`)) _karma_multiplier) 0.0 9999999.0))
  (set `self.Current Moral State` (+ (* Moral _karma_multiplier) (`self.Current Moral State`))))