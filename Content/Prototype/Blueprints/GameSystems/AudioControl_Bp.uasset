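; AudioControl_Bp is a trigger-box actor that switches ambient sound when the BP_Jin character enters it.
; On overlap, a FadeIn flag picks the behaviour for a referenced ambient sound actor.
; When set, it assigns the configured track and volume, then fades in over a few seconds; otherwise it fades the current sound out.
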(event `self.Box.OnComponentBeginOverlap`
  (params (OverlappedComponent :type "PrimitiveComponent Object Reference") (OtherActor :type "Actor Object Reference") (OtherComp :type "PrimitiveComponent Object Reference") (OtherBodyIndex :type Integer) (bFromSweep :type Boolean) (SweepResult :type "HitResult Structure (by ref)"))
  (bind _audiocomponent (`AmbientSound.AudioComponent` (`self.Ambient Sound Actor`)))
  (cast `/Game/Prototype/Blueprints/PlayerCharacter/BP_Jin` OtherActor)
  (if (`self.Fade In?`)
    (`AudioComponent.SetSound` _audiocomponent (`self.Track`))
    (`AudioComponent.SetVolumeMultiplier` _audiocomponent (`self.Volume`))
    (`AudioComponent.FadeIn` _audiocomponent 5.0 1.0 0.0)
    (else
      (`AudioComponent.FadeOut` _audiocomponent 5.0 0.0))))

(fn `UserConstructionScript`)