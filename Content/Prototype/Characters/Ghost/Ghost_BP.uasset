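; Ghost enemy that chases the player with AI MoveTo when its attention radius is entered or it takes damage.
; Tick triggers an energy-costing tackle montage while InRange; low energy makes it wander until timeline-driven regeneration refills it, then chase again.
; A separate Attack event applies damage through a forward sphere trace.
; Damage flashes a dynamic material; death spawns an explosion and random shard loot, then destroys the actor.
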(event `self.ReceiveTick`
  (params (DeltaSeconds :type "Float (single-precision)"))
  ;[1 1 1] Never Surrender
  (if (`self.IsDead`)
    _
    (elif (`self.InRange`)
      (if (>= (`self.Energy`) (`self.Attackloss`))
        (`self.Kill`)))))

(event `self.ReceiveBeginPlay`
  ;[0 1 0.5736] Energy Regeneration
  (bind (_direction _time) (`Timeline|Regeneration`)
    (:`Update`
      (if (>= _time 1.0)
        (if (< (`self.Energy`) 100.0)
          (if (`self.IsRegenerating`)
            (`self.Energy Regeneration`)
            (else
              (set `self.IsRegenerating` true))))))))

(event `Chase`
  (params (Target :type "Object Object Reference"))
  (bind _returnvalue (`GameplayStatics.GetPlayerCharacter` 0))
  ;[1 1 1] Gotta catch m all
  (if (not (`self.IsDead`))
    (`|AIMoveTo` self (`self.K2_GetActorLocation` _returnvalue) _returnvalue 50.0)))

(event `self.Attack Radius.OnComponentBeginOverlap`
  (params (OverlappedComponent :type "PrimitiveComponent Object Reference") (OtherActor :type "Actor Object Reference") (OtherComp :type "PrimitiveComponent Object Reference") (OtherBodyIndex :type Integer) (bFromSweep :type Boolean) (SweepResult :type "HitResult Structure (by ref)"))
  ;[1 1 1] Sensing
  (if (`self.IsDead`)
    (cast `/Game/Prototype/Blueprints/PlayerCharacter/BP_Jin` OtherActor)
    (set `self.InRange` true)))

(event `Kill`
  ;[1 1 1] Exterminate
  (if (not (`self.IsAttacking`))
    (`self.Energyloss`)
    (set `self.IsAttacking` true)
    (`self.PlayAnimMontage` "/Game/Prototype/Characters/Ghost/Ghost_Tackle_Montage.Ghost_Tackle_Montage")
    (`KismetSystemLibrary.Delay` 1.0)
    (if (not (>= (`self.Energy`) (`self.Attackloss`)))
      (`self.Move Away`))))

(event `self.Attack Radius.OnComponentEndOverlap`
  (params (OverlappedComponent :type "PrimitiveComponent Object Reference") (OtherActor :type "Actor Object Reference") (OtherComp :type "PrimitiveComponent Object Reference") (OtherBodyIndex :type Integer))
  ;[1 1 1] Sensing
  (if (not (`self.IsDead`))
    (set `self.InRange` false)))

(event `self.Attention Radius.OnComponentBeginOverlap`
  (params (OverlappedComponent :type "PrimitiveComponent Object Reference") (OtherActor :type "Actor Object Reference") (OtherComp :type "PrimitiveComponent Object Reference") (OtherBodyIndex :type Integer) (bFromSweep :type Boolean) (SweepResult :type "HitResult Structure (by ref)"))
  ;[1 1 1] Sensing
  (if (not (`self.IsDead`))
    (`self.Chase` OtherActor)))

(event `Move Away`
  ;[1 1 1] Run you fool
  (`|AIMoveTo` self (+ (`NavigationSystemV1.K2_GetRandomReachablePointInRadius` (`self.K2_GetActorLocation`) 500.0 null null) (`self.MinDistance`)) null
    (:`OnSuccess`
      _)
    (:`OnFail`
      _))
  (if (>= (`self.Energy`) 100.0)
    (`self.Chase` (`GameplayStatics.GetPlayerCharacter` 0))
    (else
      (`self.Move Away`))))

(event `self.ReceiveAnyDamage`
  (params (Damage :type "Float (single-precision)") (DamageType :type "DamageType Object Reference") (InstigatedBy :type "Controller Object Reference") (DamageCauser :type "Actor Object Reference"))
  (bind _mesh (`self.Mesh`))
  (bind _mesh_2 (`self.Mesh`))
  ;[1 1 1] Damage and Death
  (`|ExecutionSequence`
    (:`then_0`
      (bind _output_get (set `self.Health` (- (`self.Health`) Damage)))
      (`PrimitiveComponent.CreateDynamicMaterialInstance` _mesh_2 1 "/Game/Prototype/Characters/Ghost/M_Ghost_Inst.M_Ghost_Inst" "None")
      (bind (_direction _damage_flash) (`Timeline|Damage Timeline` :!via `PlayFromStart`)
        (:`Update`
          (`MeshComponent.SetScalarParameterValueOnMaterials` _mesh_2 "Flash" _damage_flash))))
    (:`then_1`
      (if (<= (`self.Health`) 0.0)
        (`/Engine/EditorBlueprintResources/StandardMacros.DoOnce` false
          (:`Completed`
            (set `self.IsDead` true)
            (`GameplayStatics.SpawnEmitterAtLocation` "/Game/StarterContent/Particles/P_Explosion.P_Explosion" (`self.K2_GetActorLocation`))
            (`PrimitiveComponent.SetSimulatePhysics` _mesh true)
            (`SkeletalMeshComponent.SetAllBodiesSimulatePhysics` _mesh true)
            (`PrimitiveComponent.SetCollisionEnabled` (`self.CapsuleComponent`) "NoCollision")
            (`self.Loot Drop`)
            (`self.K2_DestroyActor`)))))
    (:`then_2`
      (if (not (`self.IsChasing`))
        (`/Engine/EditorBlueprintResources/StandardMacros.DoOnce` false
          (:`Completed`
            (`self.Chase` (`GameplayStatics.GetPlayerCharacter` 0))))))))

(event `Attack`
  (bind _returnvalue (`self.K2_GetActorLocation`))
  ;[1 0 0.04893] Attack
  (bind _outhits (`KismetSystemLibrary.SphereTraceMulti` _returnvalue (+ _returnvalue (* (`self.GetActorForwardVector`) (`self.Range`))) 50.0 "TraceTypeQuery1" false (`|MakeArray` self :!type "Actor Object Reference")))
  (for _array_element _outhits
    (bind (_bblockinghit _binitialoverlap _time _distance _location _impactpoint _normal _impactnormal _physmat _hitactor) (`GameplayStatics.BreakHitResult` _array_element))
    (`GameplayStatics.SpawnEmitterAtLocation` "/Game/Prototype/Particles/P_splash.P_splash" _location)
    (`GameplayStatics.PlaySoundAtLocation` null _location (struct) 1.0 1.0 0.0 null null null)
    (`GameplayStatics.ApplyDamage` _hitactor (`self.Damage`) null self "/Game/Prototype/Blueprints/AI/BaseDamage.BaseDamage_C")))

(fn `Energy Regeneration`
  (bind _output_get (set `self.Energy` (+ (`self.Energy`) 10.0))))

(fn `Energyloss`
  (set `self.Energy` (- (`self.Energy`) (`self.Attackloss`)))
  (set `self.IsRegenerating` false))

(fn `Loot Drop`
  (for _ (range (+ (`KismetMathLibrary.RandomIntegerInRange` (`self.Min Loot`) (`self.Max Loot`)) 1))
    (`|SpawnActorFromClass` "/Game/Prototype/Blueprints/WorldInteractive/Shard_BP.Shard_BP_C" (`self.GetTransform`) "AlwaysSpawn" "OverrideRootScale" null null)))

(fn `UserConstructionScript`)